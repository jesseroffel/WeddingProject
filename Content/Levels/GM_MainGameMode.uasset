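; Main game mode that runs a timed local multiplayer match from start through finish and restart.
; BeginPlay finds the camera, progression and cat manager actors, spawns players at tag-numbered PlayerStarts on a shared camera, and creates the HUD.
; A voicemail timer delays gameplay and the clock.
; Finishing blocks input, shows results, saves faster times asynchronously to a highscore SaveGame, and enables restart after a delay.
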(event Custom|FinishGame
  ;[1 1 1] Finish Game
  (Default|ObjectiveUpdateHUD (Variables|Game|GetmyHudReference) "NewEnumerator11" true)
  (for _array_element (Variables|Spawning|GetPlayerBaseArray)
    (Default|SetInputBlocked _array_element true))
  (Variables|Default|SetmyGameRunning false)
  (Default|HandleFinishGame (Variables|Game|GetmyProgression))
  (bind _returnvalue (UserInterface|CreateWidget "/Game/UI/W_Finish.W_Finish_C" (Game|GetPlayerController (Default|GetPlayerID (Utilities|Array|Get(acopy) (Variables|Spawning|GetPlayerBaseArray))))))
  (UserInterface|Viewport|AddtoViewport _returnvalue 0)
  (Utilities|Time|SetTimerbyEvent (delegate Custom|ShowRestartText) 11.3)
  (bind _highscore (CallFunction|HandleAchieveTime _returnvalue))
  (if _highscore
    (if (not (Utilities|IsValid (Variables|Default|GetmySavegame)))
      (bind _returnvalue_2 (SaveGame|CreateSaveGameObject "/Game/Blueprints/SG_SaveGame.SG_SaveGame_C"))
      (Variables|Default|SetmySavegame _returnvalue_2))
    (Variables|/Game/Blueprints/SG_SaveGame.SG_SaveGame_C|SetTimeHighscore (Variables|Default|GetmySavegame) (Variables|Default|GetmyHighScoreTime))
    (|AsyncSaveGametoSlot (Variables|Default|GetmySavegame) (Variables|/Game/Blueprints/SG_SaveGame.SG_SaveGame_C|GetSaveSlotName (Variables|Default|GetmySavegame)) (Variables|/Game/Blueprints/SG_SaveGame.SG_SaveGame_C|GetUserIndex (Variables|Default|GetmySavegame)))))

(event Custom|ObjectiveUpdateHUD
  (params (ObjectiveType :type E_ObjectiveType%20Enum :default "NewEnumerator0") (IsComplete :type Boolean))
  ;[1 1 1] Objective Update HUD
  (Default|ObjectiveUpdateHUD (Variables|Game|GetmyHudReference) ObjectiveType IsComplete))

(event Custom|ShowRestartText
  ;[1 1 1] Finish Game
  (Variables|Default|SetmyRestartEnabled true)
  (Default|ShowRestartButton (stale Custom|FinishGame _returnvalue)))

(event Custom|VoicemailWaitOver
  ;[1 1 1] Begin Game
  (Variables|Default|SetmyGameRunning true)
  (Default|ShowHUD (Variables|Game|GetmyHudReference))
  (Default|OnStartGame (Variables|Game|GetmyCatManager))
  (Default|StartPlayers (Variables|Game|GetmyProgression))
  (for _array_element (Variables|Spawning|GetPlayerBaseArray)
    (Default|RemoveStartingBlock _array_element)
    (Variables|Default|SetmyGameStartTime (Math|DateTime|Now))))

(event Custom|RestartGame
  ;[1 1 1] Restart Game
  (Variables|Default|SetmyRestartEnabled false)
  (Game|OpenLevel(byObjectReference) "/Game/Levels/L_Home.L_Home")
  (Variables|Default|SetmyGameRunning false))

(event EventBeginPlay
  ;[1 1 1] Begin Game
  (CallFunction|SetupCamera)
  (CallFunction|SetupProgression)
  (CallFunction|SetupCatManager)
  (Utilities|FlowControl|Delay 0.21)
  (CallFunction|SetupPlayerPositions)
  (bind _returnvalue (UserInterface|CreateWidget "/Game/UI/W_HUD.W_HUD_C" (Game|GetPlayerController (Default|GetPlayerID (Utilities|Array|Get(acopy) (Variables|Spawning|GetPlayerBaseArray))))))
  (Variables|Game|SetmyHudReference _returnvalue)
  (UserInterface|Viewport|AddtoViewport _returnvalue 0)
  (Default|StartGame (Variables|Game|GetmyProgression))
  (Utilities|Time|SetTimerbyEvent (delegate Custom|VoicemailWaitOver) (Variables|Default|GetmyVoicemailWaitTimer))
  (bind (_savegame _bsuccess) (|AsyncLoadGamefromSlot "HighscoreSaveSlot")
    (:Completed
      (if _bsuccess
        (bind _assg_save_game (Utilities|Casting|CastToSG_SaveGame _savegame))
        (bind _output_get (Variables|Default|SetmySavegame _assg_save_game))
        (bind _output_get_2 (Variables|Default|SetmyHighScoreTime (Variables|/Game/Blueprints/SG_SaveGame.SG_SaveGame_C|GetTimeHighscore _output_get)))
        (Development|PrintString (Utilities|String|Append "Found highscore: " (Utilities|String|ToString(Text) (Class|KismetTextLibrary|AsTimespanTimespan _output_get_2))))
        (else
          (Variables|Default|SetmyHighScoreTime ""))))))

(fn ConstructionScript)

(fn SpawnCharacters
  (for (_ _array_index) (Variables|Spawning|GetPlayerStartArray)
    (LocalVariables|SetIndex _array_index)
    (for _array_element (Variables|Spawning|GetPlayerStartArray)
      (if (== (CallFunction|NametoInt _array_element) (+ (LocalVariables|GetIndex) 1))
        (bind _returnvalue (Class|GameplayStatics|CreatePlayer -1))
        (bind _returnvalue_2 (Game|SpawnActorfromClass "/Game/Blueprints/BP_PlayerBase.BP_PlayerBase_C" (Transformation|GetActorTransform (Utilities|Array|Get(acopy) (Variables|Spawning|GetPlayerStartArray) (LocalVariables|GetIndex))) "Undefined" _returnvalue (Utilities|Select :Index (LocalVariables|GetcontrollerIndex) :Option%200 "NewEnumerator1" :Option%201 "NewEnumerator2") (Class|GameplayStatics|GetPlayerControllerID _returnvalue) 0))
        (Utilities|Array|AddUnique (Variables|Spawning|GetPlayerBaseArray) _returnvalue_2)
        (Pawn|Possess (Game|GetPlayerController (LocalVariables|GetIndex)) _returnvalue_2)
        (Utilities|Array|AddUnique (Variables|Spawning|GetPlayerControllerArray) (Game|GetPlayerController (LocalVariables|GetIndex)))
        (Game|Player|SetViewTargetwithBlend (Game|GetPlayerController (LocalVariables|GetIndex)) (Variables|Game|GetmyGameCamera) 0.0 "VTBlend_Linear" 0.0 false)
        (Math|Integer|IncrementInt (LocalVariables|GetcontrollerIndex))))))

(fn NametoInt
  (params (PlayerStart :type Player%20Start%20Object%20Reference))
  (return (Math|Conversions|ToInteger(Byte) (Utilities|String|ToString(Name) (Variables|/Script/Engine.PlayerStart|GetPlayerStartTag PlayerStart)))))

(fn SetupCamera
  (bind _outactors (Actor|GetAllActorsOfClass "/Game/Blueprints/BP_GameCamera.BP_GameCamera_C"))
  (if (!= (Utilities|Array|Length _outactors) 0)
    (Variables|Game|SetmyGameCamera (Utilities|Array|Get(acopy) _outactors))
    (Game|Player|SetViewTargetwithBlend (Game|GetPlayerController 0) (Variables|Game|GetmyGameCamera) 0.0 "VTBlend_Linear" 0.0 false))
  (return))

(fn SetupProgression
  (bind _outactors (Actor|GetAllActorsOfClass "/Game/Blueprints/BP_Progression.BP_Progression_C"))
  (if (!= (Utilities|Array|Length _outactors) 0)
    (Variables|Game|SetmyProgression (Utilities|Array|Get(acopy) _outactors)))
  (return))

(fn SetupPlayerPositions
  (bind _outactors (Actor|GetAllActorsOfClass "/Script/Engine.PlayerStart"))
  (Variables|Spawning|SetPlayerStartArray _outactors)
  (CallFunction|SpawnCharacters)
  (Default|SetupCamera (Variables|Game|GetmyGameCamera) (Variables|Spawning|GetPlayerBaseArray)))

(fn IsGameRunning
  (return (Variables|Default|GetmyGameRunning)))

(fn GetMusicVolume
  (params (Suppressed :type Boolean))
  (if Suppressed
    (return (Variables|Default|GetmyMusicSuppressedVolume))
    (else
      (return (Variables|Default|GetmyMusicNormalVolume)))))

(fn GetSFXVolume
  (return (Variables|Default|GetmySoundEffectVolume)))

(fn SetupCatManager
  (bind _outactors (Actor|GetAllActorsOfClass "/Game/Blueprints/BP_CatManager.BP_CatManager_C"))
  (if (!= (Utilities|Array|Length _outactors) 0)
    (Variables|Game|SetmyCatManager (Utilities|Array|Get(acopy) _outactors)))
  (return))

(fn HandleAchieveTime
  (params (FinishWidget :type W%20Finish%20Object%20Reference))
  (bind _returnvalue (Math|DateTime|Now))
  (bind _mygamestarttime (Variables|Default|GetmyGameStartTime))
  (bind _returnvalue_2 (- _returnvalue _mygamestarttime))
  (if (< _returnvalue_2 (Variables|Default|GetmyHighScoreTime))
    (LocalVariables|SetSetHighscore true)
    (Variables|Default|SetmyHighScoreTime _returnvalue_2)
    (Development|PrintString "Faster time!"))
  (Default|DisplayTimes FinishWidget _returnvalue_2 (Variables|Default|GetmyHighScoreTime))
  (return (LocalVariables|GetSetHighscore)))

(fn GetRestartEnabled
  (return (Variables|Default|GetmyRestartEnabled)))

(fn SpawnPlayer
  (params (CurrentPlayerIndex :type Integer) (InputReceiver :type BP%20Input%20Receiver%20Object%20Reference)))