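; BP_ButtonMashInteraction is an interaction that players complete by repeatedly pressing a gamepad face button, randomly picked in the construction script.
; A collision sphere reports players entering and leaving to inherited handlers, disabling itself when one leaves after completion.
; TriggerInteract counts matching presses, calls the parent logic and changes the interaction state at the required count, printing progress on screen.
; Getters expose the key and press counts.
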(event OnComponentBeginOverlap(SphereCollision)
  (params (OverlappedComponent :type Primitive%20Component%20Object%20Reference) (OtherActor :type Actor%20Object%20Reference) (OtherComp :type Primitive%20Component%20Object%20Reference) (OtherBodyIndex :type Integer) (bFromSweep :type Boolean) (SweepResult :type Hit%20Result%20Structure%20%28by%20ref%29))
  (bind _asbp_player_base (Utilities|Casting|CastToBP_PlayerBase OtherActor))
  (CallFunction|OnPlayerBeginOverlap _asbp_player_base))

(event OnComponentEndOverlap(SphereCollision)
  (params (OverlappedComponent :type Primitive%20Component%20Object%20Reference) (OtherActor :type Actor%20Object%20Reference) (OtherComp :type Primitive%20Component%20Object%20Reference) (OtherBodyIndex :type Integer))
  (bind _asbp_player_base (Utilities|Casting|CastToBP_PlayerBase OtherActor))
  (CallFunction|OnPlayerEndOverlap _asbp_player_base)
  (if (CallFunction|IsCompleted)
    (Collision|SetCollisionEnabled (Variables|Default|GetSphereCollision) "NoCollision")))

(fn ConstructionScript
  (|CallParentFunction)
  (Variables|Default|SetmyInteractionType "NewEnumerator1")
  (Variables|ButtonMash|SetmyButtonMashKey (Utilities|Select :Index (Math|Random|RandomIntegerinRange 0 3) :Option%200 "Gamepad_FaceButton_Bottom" :Option%201 "Gamepad_FaceButton_Right" :Option%202 "Gamepad_FaceButton_Top" :Option%203 "Gamepad_FaceButton_Left")))

(fn OnCompleted
  (|CallParentFunction)
  (Development|PrintString "BP_StationaryInteraction Finished!"))

(fn TriggerInteract
  (params (PressedInput :type Key%20Structure :default "None"))
  (bind _myrequiredinputpresses (Variables|ButtonMash|GetmyRequiredInputPresses))
  (bind _mycurrentinputpresses (Variables|ButtonMash|GetmyCurrentInputPresses))
  (bind _returnvalue (>= _mycurrentinputpresses _myrequiredinputpresses))
  (if _returnvalue
    (Development|PrintString "Already Finished")
    (return true true)
    (elif (== PressedInput (Variables|ButtonMash|GetmyButtonMashKey))
      (Math|Integer|IncrementInt (Variables|ButtonMash|GetmyCurrentInputPresses)
        (:%20%20
          (Development|PrintString (Utilities|String|Append (Utilities|String|ToString(Integer) (Variables|ButtonMash|GetmyCurrentInputPresses)) " / " (Utilities|String|ToString(Integer) (Variables|ButtonMash|GetmyRequiredInputPresses))))
          (|CallParentFunction PressedInput)
          (if _returnvalue
            (CallFunction|SetInteractionState "NewEnumerator5")
            (return true true)
            (else
              (return true false))))))))

(fn GetButtonMashKey
  (return (Variables|ButtonMash|GetmyButtonMashKey)))

(fn GetRequiredInputPressed
  (return (Variables|ButtonMash|GetmyRequiredInputPresses) (Variables|ButtonMash|GetmyCurrentInputPresses)))