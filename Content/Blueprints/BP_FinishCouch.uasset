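; Finish couch that ends the game once two players are seated on it after all but one of the progression interactables are completed.
; Tick polls BP_Progression to toggle both seat trigger boxes, then calls FinishGame on GM_MainGameMode when both players sit.
; Each box claims a distinct cat-holding player, passes it a couch reference and shows a widget.
; Sit and stand requests move claimed players to their seat's transforms.
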(event OnComponentBeginOverlap(BoxP1)
  (params (OverlappedComponent :type Primitive%20Component%20Object%20Reference) (OtherActor :type Actor%20Object%20Reference) (OtherComp :type Primitive%20Component%20Object%20Reference) (OtherBodyIndex :type Integer) (bFromSweep :type Boolean) (SweepResult :type Hit%20Result%20Structure%20%28by%20ref%29))
  ;[1 1 1] On Begin / End Overlap P1
  (bind _asbp_player_base (Utilities|Casting|CastToBP_PlayerBase OtherActor))
  (if (Math|Boolean|ANDBoolean (Default|GetIsHoldingCat _asbp_player_base) (not (Utilities|IsValid (Variables|Default|GetmyInteractingP1))) (!= _asbp_player_base (Variables|Default|GetmyInteractingP2)))
    (bind _output_get (Variables|Default|SetmyInteractingP1 _asbp_player_base))
    (Default|SetCouchRef _output_get self)
    (Development|SetHiddeninGame (Variables|Default|GetWidget) false false)))

(event OnComponentEndOverlap(BoxP1)
  (params (OverlappedComponent :type Primitive%20Component%20Object%20Reference) (OtherActor :type Actor%20Object%20Reference) (OtherComp :type Primitive%20Component%20Object%20Reference) (OtherBodyIndex :type Integer))
  ;[1 1 1] On Begin / End Overlap P1
  (bind _asbp_player_base (Utilities|Casting|CastToBP_PlayerBase OtherActor))
  (if (== _asbp_player_base (Variables|Default|GetmyInteractingP1))
    (if (not (Default|GetIsSitting (Variables|Default|GetmyInteractingP1)))
      (Default|SetCouchRef (Variables|Default|GetmyInteractingP1))
      (Variables|Default|SetmyInteractingP1 0)
      (Development|SetHiddeninGame (Variables|Default|GetWidget) true false))))

(event OnComponentBeginOverlap(BoxP2)
  (params (OverlappedComponent :type Primitive%20Component%20Object%20Reference) (OtherActor :type Actor%20Object%20Reference) (OtherComp :type Primitive%20Component%20Object%20Reference) (OtherBodyIndex :type Integer) (bFromSweep :type Boolean) (SweepResult :type Hit%20Result%20Structure%20%28by%20ref%29))
  ;[1 1 1] On Begin / End Overlap P2
  (bind _asbp_player_base (Utilities|Casting|CastToBP_PlayerBase OtherActor))
  (if (Math|Boolean|ANDBoolean (Default|GetIsHoldingCat _asbp_player_base) (not (Utilities|IsValid (Variables|Default|GetmyInteractingP2))) (!= _asbp_player_base (Variables|Default|GetmyInteractingP1)))
    (bind _output_get (Variables|Default|SetmyInteractingP2 _asbp_player_base))
    (Default|SetCouchRef _output_get self)
    (Development|SetHiddeninGame (Variables|Default|GetWidgetP2) false false)))

(event OnComponentEndOverlap(BoxP2)
  (params (OverlappedComponent :type Primitive%20Component%20Object%20Reference) (OtherActor :type Actor%20Object%20Reference) (OtherComp :type Primitive%20Component%20Object%20Reference) (OtherBodyIndex :type Integer))
  ;[1 1 1] On Begin / End Overlap P2
  (bind _asbp_player_base (Utilities|Casting|CastToBP_PlayerBase OtherActor))
  (if (== _asbp_player_base (Variables|Default|GetmyInteractingP2))
    (if (not (Default|GetIsSitting (Variables|Default|GetmyInteractingP2)))
      (Default|SetCouchRef (Variables|Default|GetmyInteractingP2))
      (Variables|Default|SetmyInteractingP2 0)
      (Development|SetHiddeninGame (Variables|Default|GetWidgetP2) true false))))

(event Custom|OnRequestCouchSit
  (params (RequestingPlayer :type BP%20Player%20Base%20Object%20Reference))
  (bind _sittransform (CallFunction|GetSitLocation RequestingPlayer))
  ;[1 1 1] On Request Sit / Stand
  (if (CallFunction|GetValidPlayerOverlap RequestingPlayer)
    (Default|SetCouchPosition RequestingPlayer (.location _sittransform) (.rotation _sittransform) true)
    (CallFunction|HideRelevantWidget RequestingPlayer)
    (else
      (Development|PrintString "ERROR: Invalid couch interaction" true true "(R=1.000000,G=0.114441,B=0.000000,A=1.000000)" 5.0))))

(event Custom|OnRequestCouchStand
  (params (RequestingPlayer :type BP%20Player%20Base%20Object%20Reference))
  (bind _returntransform (CallFunction|GetStandLocation RequestingPlayer))
  ;[1 1 1] On Request Sit / Stand
  (if (CallFunction|GetValidPlayerOverlap RequestingPlayer)
    (Default|SetCouchPosition RequestingPlayer (.location _returntransform) (.rotation _returntransform) false)
    (else
      (Development|PrintString "ERROR: Invalid couch interaction" true true "(R=1.000000,G=0.114441,B=0.000000,A=1.000000)" 5.0))))

(event EventBeginPlay
  ;[1 1 1] Begin Play
  (bind _outactors (Actor|GetAllActorsOfClass "/Game/Blueprints/BP_Progression.BP_Progression_C"))
  (if (> (Utilities|Array|Length _outactors) 0)
    (Variables|Default|SetmyProgression (Utilities|Array|Get(acopy) _outactors))
    (Actor|Tick|SetActorTickEnabled true)
    (else
      (Development|PrintString "ERROR: Cannot find BP_Progression for Finish" true true "(R=1.000000,G=0.105670,B=0.000000,A=1.000000)" 5.0))))

(event EventTick
  (params (DeltaSeconds :type Float%20%28single-precision%29))
  (bind _myprogression (Variables|Default|GetmyProgression))
  (bind (_completedinteractables _totalinteractables) (Default|GetCompletedInteractables _myprogression))
  ;[1 1 1] Event Tick
  (if (>= _completedinteractables (- _totalinteractables 1))
    (if (Variables|Default|GetmyAllInteractablesReady)
      (if (CallFunction|CanFinishGame)
        (bind _asgm_main_game_mode (Utilities|Casting|CastToGM_MainGameMode (Game|GetGameMode)))
        (Default|FinishGame _asgm_main_game_mode)
        (Actor|Tick|SetActorTickEnabled false))
      (else
        (CallFunction|SetInteractionEnabled true)
        (Development|PrintString "Can finish game!")))
    (elif (Variables|Default|GetmyAllInteractablesReady)
      (CallFunction|SetInteractionEnabled false))))

(fn ConstructionScript
  (|CallParentFunction)
  (CallFunction|SetInteractionEnabled false))

(fn CanFinishGame
  (if (Math|Boolean|ANDBoolean (Variables|Default|GetmyAllInteractablesReady) (Utilities|IsValid (Variables|Default|GetmyInteractingP1)) (Utilities|IsValid (Variables|Default|GetmyInteractingP2)))
    (return (and (Default|GetIsSitting (Variables|Default|GetmyInteractingP1)) (Default|GetIsSitting (Variables|Default|GetmyInteractingP2))))
    (else
      (return false))))

(fn SetInteractionEnabled
  (params (IsEnabled :type Boolean))
  (if IsEnabled
    (Collision|SetCollisionEnabled (Variables|Default|GetBoxP1) "QueryAndPhysics")
    (Collision|SetCollisionEnabled (Variables|Default|GetBoxP2) "QueryAndPhysics")
    (Variables|Default|SetmyAllInteractablesReady true)
    (else
      (Collision|SetCollisionEnabled (Variables|Default|GetBoxP1) "NoCollision")
      (Collision|SetCollisionEnabled (Variables|Default|GetBoxP2) "NoCollision")
      (Variables|Default|SetmyAllInteractablesReady false))))

(fn GetValidPlayerOverlap
  (params (RequestingPlayer :type BP%20Player%20Base%20Object%20Reference))
  (return (or (== RequestingPlayer (Variables|Default|GetmyInteractingP1)) (== RequestingPlayer (Variables|Default|GetmyInteractingP2)))))

(fn GetSitLocation
  (params (RequestingPlayer :type BP%20Player%20Base%20Object%20Reference))
  (if (== RequestingPlayer (Variables|Default|GetmyInteractingP1))
    (return (Transformation|GetWorldTransform (Variables|Default|GetSitLocationP1)))
    (else
      (return (Transformation|GetWorldTransform (Variables|Default|GetSitLocationP2))))))

(fn GetStandLocation
  (params (RequestingPlayer :type BP%20Player%20Base%20Object%20Reference))
  (if (== RequestingPlayer (Variables|Default|GetmyInteractingP1))
    (return (Transformation|GetWorldTransform (Variables|Default|GetStandLocationP1)))
    (else
      (return (Transformation|GetWorldTransform (Variables|Default|GetStandLocationP2))))))

(fn HideRelevantWidget
  (params (RequestingPlayer :type BP%20Player%20Base%20Object%20Reference))
  (if (== RequestingPlayer (Variables|Default|GetmyInteractingP1))
    (Development|SetHiddeninGame (Variables|Default|GetWidget) true false)
    (else
      (Development|SetHiddeninGame (Variables|Default|GetWidgetP2) true false))))