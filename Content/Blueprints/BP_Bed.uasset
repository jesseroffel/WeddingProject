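; BP_Bed is an interactable bed that the player completes as an objective in the main game mode.
; It hands its box collision to inherited interaction logic and forwards overlap begin and end events to it.
; Starting interaction plays a fabric-folding sound.
; Completion stops the audio, swaps the mesh to a completed bed and tells GM_MainGameMode to mark the objective complete on the HUD.
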(event OnComponentBeginOverlap(BoxCollision)
  (params (OverlappedComponent :type Primitive%20Component%20Object%20Reference) (OtherActor :type Actor%20Object%20Reference) (OtherComp :type Primitive%20Component%20Object%20Reference) (OtherBodyIndex :type Integer) (bFromSweep :type Boolean) (SweepResult :type Hit%20Result%20Structure%20%28by%20ref%29))
  (CallFunction|OnBeginOverlap OtherActor))

(event OnComponentEndOverlap(BoxCollision)
  (params (OverlappedComponent :type Primitive%20Component%20Object%20Reference) (OtherActor :type Actor%20Object%20Reference) (OtherComp :type Primitive%20Component%20Object%20Reference) (OtherBodyIndex :type Integer))
  (CallFunction|OnEndOverlap OtherActor))

(event EventBeginPlay
  (Variables|Default|SetmyBoxCollision (Variables|Default|GetBoxCollision)))

(fn ConstructionScript
  (|CallParentFunction))

(fn OnInteractionStart
  (Audio|Components|Audio|SetSound (Variables|Default|GetAudio) "/Game/Audio/SFX/SQ_Folding_Fabric.SQ_Folding_Fabric")
  (Audio|Components|Audio|Play (Variables|Default|GetAudio) 0.0))

(fn OnInteractionCompleted
  (|CallParentFunction)
  (Audio|Components|Audio|Stop (Variables|Default|GetAudio))
  (Components|StaticMesh|SetStaticMesh (Variables|Default|GetBedModel) "/Game/Props/Interactable/SM_Bed_completed.SM_Bed_completed")
  (bind _asgm_main_game_mode (Utilities|Casting|CastToGM_MainGameMode (Game|GetGameMode)))
  (Default|ObjectiveUpdateHUD _asgm_main_game_mode "NewEnumerator7" true))