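; BP_WashDishes is a dish-washing interactable that turns a dirty plate stack into clean dishes through repeated input presses.
; It builds on a parent interaction class, forwarding box overlaps and extending the start, trigger and completion steps.
; Each press maps progress to quarter-based mesh stages, swapping the dirty and clean stacks in opposite order.
; Starting plays plate audio; completion stops it, hides both stacks and spawns BP_CleanDishes at the clean stack.
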(event OnComponentBeginOverlap(BoxCollision)
  (params (OverlappedComponent :type Primitive%20Component%20Object%20Reference) (OtherActor :type Actor%20Object%20Reference) (OtherComp :type Primitive%20Component%20Object%20Reference) (OtherBodyIndex :type Integer) (bFromSweep :type Boolean) (SweepResult :type Hit%20Result%20Structure%20%28by%20ref%29))
  (CallFunction|OnBeginOverlap OtherActor))

(event OnComponentEndOverlap(BoxCollision)
  (params (OverlappedComponent :type Primitive%20Component%20Object%20Reference) (OtherActor :type Actor%20Object%20Reference) (OtherComp :type Primitive%20Component%20Object%20Reference) (OtherBodyIndex :type Integer))
  (CallFunction|OnEndOverlap OtherActor))

(event EventBeginPlay
  (Variables|Default|SetmyBoxCollision (Variables|Default|GetBoxCollision)))

(fn ConstructionScript
  (|CallParentFunction))

(fn OnInteractionCompleted
  (bind _cleandishes (Variables|Default|GetCleanDishes))
  (bind _returnvalue (Transformation|GetWorldTransform _cleandishes))
  (|CallParentFunction)
  (Audio|Components|Audio|Stop (Variables|Default|GetAudio))
  (Game|SpawnActorfromClass "/Game/Blueprints/BP_CleanDishes.BP_CleanDishes_C" (Math|Transform|MakeTransform (.location _returnvalue) (.rotation _returnvalue) "1,1,1") "AlwaysSpawn" 0 0)
  (Rendering|SetVisibility (Variables|Default|GetCleanDishes) false false)
  (Rendering|SetVisibility (Variables|Default|GetDirtyDishes) false false))

(fn TriggerInteract
  (params (PressedInput :type Key%20Structure))
  (bind (_success _finished) (|CallParentFunction PressedInput))
  (CallFunction|SwitchPlates)
  (return _success _finished))

(fn SwitchPlates
  (bind _output_get (LocalVariables|SetcurrentPercentage (/ (Math|Conversions|ToFloat(Integer) (Variables|Default|GetmyCurrentInputPresses)) (Math|Conversions|ToFloat(Integer) (Variables|Default|GetmyRequiredInputPresses)))))
  (if (<= _output_get 0.75)
    (if (<= (LocalVariables|GetcurrentPercentage) 0.5)
      (if (<= (LocalVariables|GetcurrentPercentage) 0.25)
        (Components|StaticMesh|SetStaticMesh (Variables|Default|GetDirtyDishes) "/Game/Props/Interactable/SM_Plate_incompelte_stage_01.SM_Plate_incompelte_stage_01")
        (Components|StaticMesh|SetStaticMesh (Variables|Default|GetCleanDishes) "/Game/Props/Interactable/SM_Plate_incompelte_stage_04.SM_Plate_incompelte_stage_04")
        (if (and (Variables|Default|GetmyCleanHidden) (> (LocalVariables|GetcurrentPercentage) 0.0))
          (Variables|Default|SetmyCleanHidden false)
          (Rendering|SetVisibility (Variables|Default|GetCleanDishes) true false))
        (else
          (Components|StaticMesh|SetStaticMesh (Variables|Default|GetDirtyDishes) "/Game/Props/Interactable/SM_Plate_incompelte_stage_02.SM_Plate_incompelte_stage_02")
          (Components|StaticMesh|SetStaticMesh (Variables|Default|GetCleanDishes) "/Game/Props/Interactable/SM_Plate_incompelte_stage_03.SM_Plate_incompelte_stage_03")))
      (else
        (Components|StaticMesh|SetStaticMesh (Variables|Default|GetDirtyDishes) "/Game/Props/Interactable/SM_Plate_incompelte_stage_03.SM_Plate_incompelte_stage_03")
        (Components|StaticMesh|SetStaticMesh (Variables|Default|GetCleanDishes) "/Game/Props/Interactable/SM_Plate_incompelte_stage_02.SM_Plate_incompelte_stage_02")))
    (else
      (Components|StaticMesh|SetStaticMesh (Variables|Default|GetDirtyDishes) "/Game/Props/Interactable/SM_Plate_incompelte_stage_04.SM_Plate_incompelte_stage_04")
      (Components|StaticMesh|SetStaticMesh (Variables|Default|GetCleanDishes) "/Game/Props/Interactable/SM_Plate_incompelte_stage_01.SM_Plate_incompelte_stage_01"))))

(fn OnInteractionStart
  (|CallParentFunction)
  (Audio|Components|Audio|SetSound (Variables|Default|GetAudio) "/Game/Audio/SFX/SQ_PlatesMoving.SQ_PlatesMoving")
  (Audio|Components|Audio|Play (Variables|Default|GetAudio) 0.0))