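; BP_CatPoint is a point that detects when the cat assigned to it arrives.
; AssignCat stores a valid cat and enables query-only collision on the Sphere.
; When that cat begins overlapping and MyWalkPoint is true, the point calls OnReachedWalkPoint on the cat.
; It then runs Reset, which switches the sphere's collision off until another assignment.
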(event OnComponentBeginOverlap(Sphere)
  (params (OverlappedComponent :type Primitive%20Component%20Object%20Reference) (OtherActor :type Actor%20Object%20Reference) (OtherComp :type Primitive%20Component%20Object%20Reference) (OtherBodyIndex :type Integer) (bFromSweep :type Boolean) (SweepResult :type Hit%20Result%20Structure%20%28by%20ref%29))
  (bind _myassignedcat (Variables|Default|GetmyAssignedCat))
  (bind _asbp_cat_base (Utilities|Casting|CastToBP_CatBase OtherActor))
  (if (== _asbp_cat_base _myassignedcat)
    (if (Variables|Default|GetmyWalkPoint)
      (Default|OnReachedWalkPoint _myassignedcat)
      (CallFunction|Reset))))

(fn ConstructionScript)

(fn AssignCat
  (params (Assigned%20Cat :type BP%20Cat%20Base%20Object%20Reference))
  (if (Utilities|IsValid Assigned%20Cat)
    (Variables|Default|SetmyAssignedCat Assigned%20Cat)
    (Collision|SetCollisionEnabled (Variables|Default|GetSphere) "QueryOnly")))

(fn Reset
  (Collision|SetCollisionEnabled (Variables|Default|GetSphere) "NoCollision"))