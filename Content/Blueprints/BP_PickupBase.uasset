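; Base pickup Blueprint that shows an interaction widget when a player comes within range.
; Sphere overlaps track one BP_PlayerBase at a time, showing the widget on entry and clearing it when that player leaves.
; SetAtDestination flags the item so the widget stops appearing on later overlaps.
; OnPickup hides the widget in game, while OnDropped is an empty function.
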(event OnComponentBeginOverlap(Sphere)
  (params (OverlappedComponent :type Primitive%20Component%20Object%20Reference) (OtherActor :type Actor%20Object%20Reference) (OtherComp :type Primitive%20Component%20Object%20Reference) (OtherBodyIndex :type Integer) (bFromSweep :type Boolean) (SweepResult :type Hit%20Result%20Structure%20%28by%20ref%29))
  (bind _asbp_player_base (Utilities|Casting|CastToBP_PlayerBase OtherActor))
  (if (not (Utilities|IsValid (Variables|Default|GetmyInteractionPlayer)))
    (Variables|Default|SetmyInteractionPlayer _asbp_player_base)
    (CallFunction|OnPlayerBeginOverlap)))

(event OnComponentEndOverlap(Sphere)
  (params (OverlappedComponent :type Primitive%20Component%20Object%20Reference) (OtherActor :type Actor%20Object%20Reference) (OtherComp :type Primitive%20Component%20Object%20Reference) (OtherBodyIndex :type Integer))
  (bind _asbp_player_base (Utilities|Casting|CastToBP_PlayerBase OtherActor))
  (if (== _asbp_player_base (Variables|Default|GetmyInteractionPlayer))
    (CallFunction|OnPlayerEndOverlap)))

(event Custom|OnPlayerBeginOverlap
  (if (not (Variables|Default|GetmyAtDestination))
    (Rendering|SetVisibility (Variables|Default|GetWidget) true false)))

(event Custom|OnPlayerEndOverlap
  (Rendering|SetVisibility (Variables|Default|GetWidget) false false)
  (Variables|Default|SetmyInteractionPlayer 0))

(fn ConstructionScript)

(fn OnPickup
  (Development|SetHiddeninGame (Variables|Default|GetWidget) true false))

(fn SetatDestination
  (Variables|Default|SetmyAtDestination true))

(fn OnDropped)