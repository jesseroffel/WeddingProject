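; BP_StationaryInteraction is an interactable that completes after a required number of input presses.
; Its sphere overlap events show the WidgetInteraction component on begin overlap and hide it on end overlap, without filtering the overlapping actor.
; TriggerInteract increments the press count until it reaches the requirement, then changes the interaction state and reports finished.
; Calls always return success, with debug prints on completion and repeat attempts.
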(event OnComponentBeginOverlap(Sphere)
  (params (OverlappedComponent :type Primitive%20Component%20Object%20Reference) (OtherActor :type Actor%20Object%20Reference) (OtherComp :type Primitive%20Component%20Object%20Reference) (OtherBodyIndex :type Integer) (bFromSweep :type Boolean) (SweepResult :type Hit%20Result%20Structure%20%28by%20ref%29))
  (Development|SetHiddeninGame (Variables|Default|GetWidgetInteraction) false false))

(event OnComponentEndOverlap(Sphere)
  (params (OverlappedComponent :type Primitive%20Component%20Object%20Reference) (OtherActor :type Actor%20Object%20Reference) (OtherComp :type Primitive%20Component%20Object%20Reference) (OtherBodyIndex :type Integer))
  (Development|SetHiddeninGame (Variables|Default|GetWidgetInteraction) true false))

(event EventBeginPlay
  (|CallParentFunction) ; This node is disabled and will not be called.\nDrag off pins to build functionality.
)

(event Collision|EventActorBeginOverlap
  (params (OtherActor :type Actor%20Object%20Reference))
  (|CallParentFunction OtherActor) ; This node is disabled and will not be called.\nDrag off pins to build functionality.
)

(event EventTick
  (params (DeltaSeconds :type Float%20%28single-precision%29))
  (|CallParentFunction DeltaSeconds) ; This node is disabled and will not be called.\nDrag off pins to build functionality.
)

(fn ConstructionScript
  (|CallParentFunction))

(fn TriggerInteract
  (bind _myrequiredinputpresses (Variables|Default|GetmyRequiredInputPresses))
  (bind _mycurrentinputpresses (Variables|Default|GetmyCurrentInputPresses))
  (bind _returnvalue (>= _mycurrentinputpresses _myrequiredinputpresses))
  (if _returnvalue
    (Development|PrintString "Already Finished")
    (return true true)
    (else
      (Math|Integer|IncrementInt (Variables|Default|GetmyCurrentInputPresses)
        (:%20%20
          (if _returnvalue
            (Variables|Default|SetmyCurrentInteractionState "NewEnumerator5")
            (Development|PrintString "BP_StationaryInteraction Finished!")
            (return true true)
            (else
              (return true false))))))))