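; Interactable cat bowl that players fill with food to attract cats, built on a parent interaction class.
; A cat manager enables the player trigger sphere, and completing the interaction disables it, swaps to the filled mesh and starts a sound-length timer.
; CatFoodDone plays meows and passes the bowl and two cat points to the manager.
; Cats entering CatSphere start eating, and OnCatsAteFood disables that sphere and restores the incomplete mesh.
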(event OnComponentBeginOverlap(SphereCollision)
  (params (OverlappedComponent :type Primitive%20Component%20Object%20Reference) (OtherActor :type Actor%20Object%20Reference) (OtherComp :type Primitive%20Component%20Object%20Reference) (OtherBodyIndex :type Integer) (bFromSweep :type Boolean) (SweepResult :type Hit%20Result%20Structure%20%28by%20ref%29))
  (bind _asbp_player_base (Utilities|Casting|CastToBP_PlayerBase OtherActor))
  (CallFunction|OnBeginOverlap _asbp_player_base))

(event OnComponentEndOverlap(SphereCollision)
  (params (OverlappedComponent :type Primitive%20Component%20Object%20Reference) (OtherActor :type Actor%20Object%20Reference) (OtherComp :type Primitive%20Component%20Object%20Reference) (OtherBodyIndex :type Integer))
  (bind _asbp_player_base (Utilities|Casting|CastToBP_PlayerBase OtherActor))
  (CallFunction|OnEndOverlap _asbp_player_base))

(event OnComponentBeginOverlap(CatSphere)
  (params (OverlappedComponent :type Primitive%20Component%20Object%20Reference) (OtherActor :type Actor%20Object%20Reference) (OtherComp :type Primitive%20Component%20Object%20Reference) (OtherBodyIndex :type Integer) (bFromSweep :type Boolean) (SweepResult :type Hit%20Result%20Structure%20%28by%20ref%29))
  (bind _asbp_cat_base (Utilities|Casting|CastToBP_CatBase OtherActor))
  (if (and (Variables|Default|GetmyCatFoodActive) (not (Utilities|Array|ContainsItem (Variables|Default|GetmyAttractedCats) _asbp_cat_base)))
    (Utilities|Array|Add (Variables|Default|GetmyAttractedCats) 0)
    (Default|OnCatBowlReached _asbp_cat_base)
    (Development|PrintString "Set cat to eating")))

(event Custom|CatFoodDone
  (bind (_point1 _point2) (CallFunction|GetCatPoints))
  (Audio|Components|Audio|SetSound (Variables|Default|GetAudio) "/Game/Audio/SFX/SFX_Meow1.SFX_Meow1")
  (Audio|Components|Audio|SetSound (Variables|Default|GetMeowSpeaker) "/Game/Audio/SFX/SFX_Meow3.SFX_Meow3")
  (Audio|Components|Audio|Play (Variables|Default|GetAudio) 0.0)
  (Audio|Components|Audio|Play (Variables|Default|GetMeowSpeaker) 0.15)
  (Default|OnCatBowlActivated (Variables|Default|GetmyCatManager) self _point1 _point2)
  (Variables|Default|SetmyCatFoodActive true)
  (Collision|SetCollisionEnabled (Variables|Default|GetSphereCollision) "NoCollision"))

(event Custom|OnCatsAteFood
  (Collision|SetCollisionEnabled (Variables|Default|GetCatSphere) "NoCollision")
  (Components|StaticMesh|SetStaticMesh (Variables|Default|GetBowl) "/Game/Props/Interactable/SM_CatBowl_incomplete.SM_CatBowl_incomplete"))

(event EventBeginPlay
  (Variables|Default|SetmySphereCollision (Variables|Default|GetSphereCollision)))

(fn ConstructionScript
  (|CallParentFunction))

(fn OnInteractionStart
  (|CallParentFunction)
  (Audio|Components|Audio|SetSound (Variables|Default|GetAudio) "/Game/Audio/SFX/SQ_CatFood.SQ_CatFood")
  (Audio|Components|Audio|Play (Variables|Default|GetAudio) 0.0))

(fn OnInteractionCompleted
  (|CallParentFunction)
  (Collision|SetCollisionEnabled (Variables|Default|GetSphereCollision) "NoCollision")
  (Components|StaticMesh|SetStaticMesh (Variables|Default|GetBowl) "/Game/Props/Interactable/SM_CatBowl_completed.SM_CatBowl_completed")
  (Audio|Components|Audio|SetSound (Variables|Default|GetAudio) "/Game/Audio/SFX/SFX_CatFoodDone.SFX_CatFoodDone")
  (Audio|Components|Audio|Play (Variables|Default|GetAudio) 0.0)
  (Utilities|Time|SetTimerbyEvent (EventDispatchers|CreateEvent :!event Custom|CatFoodDone) (Variables|/Script/Engine.SoundBase|GetDuration (Variables|/Script/Engine.AudioComponent|GetSound (Variables|Default|GetAudio)))))

(fn OnCatFoodFinished
  (Components|StaticMesh|SetStaticMesh (Variables|Default|GetBowl) "/Game/Props/Interactable/SM_CatBowl_incomplete.SM_CatBowl_incomplete"))

(fn EnableFoodInteraction
  (params (CatManager :type BP%20Cat%20Manager%20Object%20Reference))
  (Variables|Default|SetmyCatManager CatManager)
  (Collision|SetCollisionEnabled (Variables|Default|GetSphereCollision) "QueryOnly")
  (Variables|Default|SetmyCatFoodActive true))

(fn GetCatPoints
  (return (Transformation|GetWorldLocation (Variables|Default|GetPoint1)) (Transformation|GetWorldLocation (Variables|Default|GetPoint2))))