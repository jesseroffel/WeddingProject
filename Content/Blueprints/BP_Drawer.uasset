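; BP_Drawer is a drawer that receives laundry pieces, built on a parent class that handles item delivery.
; On BeginPlay it sets its required item count to the number of BP_ItemLaundryPiece actors in the level.
; Each provided item plays a clothing pickup sound.
; When all items are received, it swaps to a closed drawer mesh and starts a half-second timer, apparently for the drawer-full sound.
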(event Custom|OnAllPiecesDelivered
  (bind _audio (Variables|Default|GetAudio))
  (Audio|Components|Audio|SetSound _audio "/Game/Audio/SFX/SFX_DrawerFull.SFX_DrawerFull")
  (Audio|Components|Audio|Play _audio 0.0))

(event EventBeginPlay
  (bind _outactors (Actor|GetAllActorsOfClass "/Game/Blueprints/BP_ItemLaundryPiece.BP_ItemLaundryPiece_C"))
  (Variables|Default|SetmyItemsRequired (Utilities|Array|Length _outactors)))

(fn ConstructionScript
  (|CallParentFunction))

(fn OnTotalItemsReceived
  (|CallParentFunction)
  (Components|StaticMesh|SetStaticMesh (Variables|Default|GetDrawer) "/Game/Props/Furnitures/SM_Drawer_Closed.SM_Drawer_Closed")
  (Utilities|Time|SetTimerbyEvent (EventDispatchers|CreateEvent :!event Custom|OnAllPiecesDelivered) 0.5))

(fn OnItemProvided
  (bind _audio (Variables|Default|GetAudio))
  (|CallParentFunction)
  (Audio|Components|Audio|SetSound _audio "/Game/Audio/SFX/SFX_ClothingPickup.SFX_ClothingPickup")
  (Audio|Components|Audio|Play _audio 0.0))