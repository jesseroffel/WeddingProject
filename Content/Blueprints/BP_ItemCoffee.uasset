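; BP_ItemCoffee is a coffee item that can be picked up and dropped.
; It overrides OnPickup and OnDropped, calling the parent logic first and then swapping the sound on the Audio component to play a coffee-specific pickup or place effect.
; The event graph holds only disabled placeholder events, and the construction script just calls its parent.
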(event EventBeginPlay)

(event Collision|EventActorBeginOverlap
  (params (OtherActor :type Actor%20Object%20Reference)))

(event EventTick
  (params (DeltaSeconds :type Float%20%28single-precision%29)))

(fn ConstructionScript
  (|CallParentFunction))

(fn OnPickup
  (bind _audio (Variables|Default|GetAudio))
  (|CallParentFunction)
  (Audio|Components|Audio|SetSound _audio "/Game/Audio/SFX/SFX_CoffeePickup.SFX_CoffeePickup")
  (Audio|Components|Audio|Play _audio 0.0))

(fn OnDropped
  (bind _audio (Variables|Default|GetAudio))
  (|CallParentFunction)
  (Audio|Components|Audio|SetSound _audio "/Game/Audio/SFX/SFX_CoffeePlace.SFX_CoffeePlace")
  (Audio|Components|Audio|Play _audio 0.0))