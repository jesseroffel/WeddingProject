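; BP_ItemPainting is a painting item that can be picked up and dropped, built as a child of a parent item Blueprint.
; It extends the parent's OnPickup and OnDropped by calling them first, then swapping the sound on the Audio component and playing it.
; Pickup uses a clothing pickup sound and dropping uses an item drop sound, while construction only defers to the parent.
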(fn ConstructionScript
  (|CallParentFunction))

(fn OnPickup
  (bind _audio (Variables|Default|GetAudio))
  (|CallParentFunction)
  (Audio|Components|Audio|SetSound _audio "/Game/Audio/SFX/SFX_ClothingPickup.SFX_ClothingPickup")
  (Audio|Components|Audio|Play _audio 0.0))

(fn OnDropped
  (bind _audio (Variables|Default|GetAudio))
  (|CallParentFunction)
  (Audio|Components|Audio|SetSound _audio "/Game/Audio/SFX/SFX_ItemDrop1.SFX_ItemDrop1")
  (Audio|Components|Audio|Play _audio 0.0))