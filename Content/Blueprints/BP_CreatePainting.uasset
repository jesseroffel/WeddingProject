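; Interactable station where a timed or staged interaction creates a painting item, built on a parent interaction Blueprint.
; It passes its box collision and overlap events to the inherited interaction logic.
; Starting the interaction plays a paint-stroke sound.
; Completing it stops the audio, hides the Painting component and spawns a BP_ItemPainting slightly below that component's position.
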(event OnComponentBeginOverlap(BoxCollision)
  (params (OverlappedComponent :type Primitive%20Component%20Object%20Reference) (OtherActor :type Actor%20Object%20Reference) (OtherComp :type Primitive%20Component%20Object%20Reference) (OtherBodyIndex :type Integer) (bFromSweep :type Boolean) (SweepResult :type Hit%20Result%20Structure%20%28by%20ref%29))
  (CallFunction|OnBeginOverlap OtherActor))

(event OnComponentEndOverlap(BoxCollision)
  (params (OverlappedComponent :type Primitive%20Component%20Object%20Reference) (OtherActor :type Actor%20Object%20Reference) (OtherComp :type Primitive%20Component%20Object%20Reference) (OtherBodyIndex :type Integer))
  (CallFunction|OnEndOverlap OtherActor))

(event EventBeginPlay
  (Variables|Default|SetmyBoxCollision (Variables|Default|GetBoxCollision)))

(fn ConstructionScript
  (|CallParentFunction))

(fn OnInteractionStart
  (|CallParentFunction)
  (Audio|Components|Audio|SetSound (Variables|Default|GetAudio) "/Game/Audio/SFX/SQ_PaintStrokes.SQ_PaintStrokes")
  (Audio|Components|Audio|Play (Variables|Default|GetAudio) 0.0))

(fn OnInteractionCompleted
  (bind _painting (Variables|Default|GetPainting))
  (bind _returnvalue (Transformation|GetWorldTransform _painting))
  (bind (_x _y _z) (Math|Vector|BreakVector (.location _returnvalue)))
  (|CallParentFunction)
  (Audio|Components|Audio|Stop (Variables|Default|GetAudio))
  (Rendering|SetVisibility _painting false false)
  (Game|SpawnActorfromClass "/Game/Blueprints/BP_ItemPainting.BP_ItemPainting_C" (Math|Transform|MakeTransform (Math|Vector|MakeVector _x _y (- _z 4e+01)) "0,210.000000, 0" "1,1,1") "AlwaysSpawn" 0 0))