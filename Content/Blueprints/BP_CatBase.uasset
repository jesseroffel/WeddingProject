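; Base cat character, skinned as Suki or Lily, that wanders the level, targets interaction objectives and can be picked up by players.
; Tick runs randomised wait timers; after several walks to points from BP_CatManager, it moves to an objective from the manager, then meows and calls its OnCatDestroy on arrival.
; An overlap sphere shows a widget to empty-handed players, and pickup halts AI movement and releases any targeted objective.
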(event OnComponentBeginOverlap(Sphere)
  (params (OverlappedComponent :type Primitive%20Component%20Object%20Reference) (OtherActor :type Actor%20Object%20Reference) (OtherComp :type Primitive%20Component%20Object%20Reference) (OtherBodyIndex :type Integer) (bFromSweep :type Boolean) (SweepResult :type Hit%20Result%20Structure%20%28by%20ref%29))
  ;[1 1 1] On Begin / End Overlap
  (bind _asbp_player_base (Utilities|Casting|CastToBP_PlayerBase OtherActor))
  (if (Math|Boolean|ANDBoolean (not (Variables|State|GetmyIsHeld)) (not (Variables|State|GetmyIsInteracting)) (not (Default|GetIsHoldingItem _asbp_player_base)))
    (Development|SetHiddeninGame (Variables|Default|GetWidget) false false)))

(event OnComponentEndOverlap(Sphere)
  (params (OverlappedComponent :type Primitive%20Component%20Object%20Reference) (OtherActor :type Actor%20Object%20Reference) (OtherComp :type Primitive%20Component%20Object%20Reference) (OtherBodyIndex :type Integer))
  ;[1 1 1] On Begin / End Overlap
  (Utilities|Casting|CastToBP_PlayerBase OtherActor)
  (Development|SetHiddeninGame (Variables|Default|GetWidget) true false))

(event Custom|OnCatInteractableReached
  (AI|Navigation|StopMovement (AI|GetAIController self))
  (Variables|State|SetmyIsWalking false)
  (Variables|State|SetmyIsInteracting true)
  (Collision|SetCollisionEnabled (Variables|Default|GetSphere) "NoCollision")
  (CallFunction|PlayMeowSound)
  (Utilities|Time|SetTimerbyEvent (delegate Custom|OnCatInteractFinished) 1.0)
  (Default|OnCatDestroy (Variables|Default|GetmyAssignedObjective) self))

(event Custom|OnCatInteractFinished
  (Variables|State|SetmyIsInteracting false)
  (Deciding|SetMovementWaitCooldown)
  (Deciding|RollNewRemainingMovetoActions)
  (Variables|Default|SetmyAssignedObjective 0)
  (Utilities|Time|SetTimerbyEvent (delegate Custom|OnPostInteractFinished) (+ (Variables|Movement|GetmyMovementWaitCooldown) 2.0)))

(event Custom|CheckPosition
  (bind _self self)
  (if (Math|Vector|Equal(Vector) (Variables|Default|GetmyLastLocation) (Transformation|GetWorldLocation (Variables|Collision|GetCapsuleComponent)) 1.0)
    (Development|PrintString "Cat reset")
    (bind _newlocation (Default|GetNewWalkLocation (Variables|Default|GetmyCatManager) _self))
    (AI|Navigation|MovetoLocation (AI|GetAIController _self) _newlocation -1.0 true true false true 0)))

(event Custom|OnTargettedInteractionCompleted
  (Default|OnResetObjective (Variables|Default|GetmyCatManager)))

(event Custom|OnPostInteractFinished
  (Collision|SetCollisionEnabled (Variables|Default|GetSphere) "QueryAndPhysics"))

(event EventBeginPlay
  (bind _mesh (Variables|Character|GetMesh))
  (switch Utilities|FlowControl|Switch|SwitchonE_CatType (Variables|State|GetmyCatType)
    (:NewEnumerator1
      (Rendering|Material|SetMaterial _mesh 0 "/Game/Characters/MI_Suki.MI_Suki"))
    (:NewEnumerator2
      (Rendering|Material|SetMaterial _mesh 0 "/Game/Characters/MI_Lily.MI_Lily")))
  (Deciding|SetMovementWaitCooldown)
  (Deciding|RollNewRemainingMovetoActions)
  (bind _outactors (Actor|GetAllActorsOfClass "/Game/Blueprints/BP_CatManager.BP_CatManager_C"))
  (if (> (Utilities|Array|Length _outactors) 0)
    (Variables|Default|SetmyCatManager (Utilities|Array|Get(acopy) _outactors))))

(event EventTick
  (params (DeltaSeconds :type Float%20%28single-precision%29))
  (CallFunction|HandleMeowCooldown DeltaSeconds)
  (CallFunction|HandleMovementDecisions DeltaSeconds))

(fn ConstructionScript)

(fn GetCatType
  (return (Variables|State|GetmyCatType)))

(fn GetIsWalking
  (return (Variables|State|GetmyIsWalking)))

(fn GetIsInteracting
  (return (Variables|State|GetmyIsInteracting)))

(fn PickedUp
  (params (HoldingPlayerRef :type BP%20Player%20Base%20Object%20Reference))
  (Variables|State|SetmyIsHeld true)
  (Variables|State|SetmyIsWalking false)
  (AI|Navigation|StopMovement (AI|GetAIController self))
  (Development|SetHiddeninGame (Variables|Default|GetWidget) true false)
  (Collision|SetCollisionEnabled (Variables|Collision|GetCapsuleComponent) "NoCollision")
  (CallFunction|CancelMovetoPoint)
  (if (Utilities|IsValid (Variables|Default|GetmyHolderPlayerRef))
    (Default|OnPassedCat (Variables|Default|GetmyHolderPlayerRef)))
  (Variables|Default|SetmyHolderPlayerRef HoldingPlayerRef)
  (if (Utilities|IsValid (Variables|Default|GetmyAssignedObjective))
    (Default|SetIsTargetted (Variables|Default|GetmyAssignedObjective) false)
    (Variables|Default|SetmyAssignedObjective 0))
  (if (<= (Variables|Meow|GetmyMeowCooldown) 0.0)
    (CallFunction|PlayMeowSound)
    (Deciding|RollNewRemainingMovetoActions)))

(fn GetIsHeld
  (return (Variables|State|GetmyIsHeld)))

(fn HandleMeowCooldown
  (params (DeltaTime :type Float%20%28single-precision%29))
  (if (> (Variables|Meow|GetmyMeowCooldown) 0.0)
    (Variables|Meow|SetmyMeowCooldownTimer (+ (Variables|Meow|GetmyMeowCooldownTimer) DeltaTime))
    (if (> (Variables|Meow|GetmyMeowCooldownTimer) (Variables|Meow|GetmyMeowCooldown))
      (Variables|Meow|SetmyMeowCooldown 0.0))))

(fn Released
  (Variables|State|SetmyIsHeld false)
  (Variables|Default|SetmyHolderPlayerRef 0)
  (Collision|SetCollisionEnabled (Variables|Collision|GetCapsuleComponent) "QueryAndPhysics"))

(fn RollNewRemainingMovetoActions
  (Variables|Movement|SetmyRemainingMoveToActions (Math|Random|RandomIntegerinRange 3 5)))

(fn HandleMovementDecisions
  (params (DeltaTime :type Float%20%28single-precision%29))
  (bind _self self)
  (if (Math|Boolean|ANDBoolean (not (Variables|State|GetmyIsWalking)) (not (Variables|State|GetmyIsHeld)) (not (Variables|State|GetmyMovementBlocked)))
    (if (not (Utilities|IsValid (Variables|Default|GetmyAssignedObjective)))
      (bind _output_get (Variables|Movement|SetmyMovementWaitTimer (+ DeltaTime (Variables|Movement|GetmyMovementWaitTimer))))
      (if (> _output_get (Variables|Movement|GetmyMovementWaitCooldown))
        (if (> (Variables|Movement|GetmyRemainingMoveToActions) 0)
          (Development|PrintString "MoveToAction")
          (else
            (bind _assignedobjective (Default|GetInteractionObjective (Variables|Default|GetmyCatManager) self))
            (if (Utilities|IsValid _assignedobjective)
              (bind _output_get_2 (Variables|Default|SetmyAssignedObjective _assignedobjective))
              (Default|OnCatTargetted _output_get_2)
              (AI|Navigation|MovetoLocation (AI|GetAIController self) (Default|GetCollisionLocation _output_get_2) -1.0 false true false true 0)
              (Variables|State|SetmyIsWalking true)
              (return)
              (else
                (Development|PrintString "No objective, walk more")
                (Deciding|SetMovementWaitCooldown)
                (Deciding|RollNewRemainingMovetoActions)))))
        (bind _newlocation (Default|GetNewWalkLocation (Variables|Default|GetmyCatManager) _self))
        (AI|Navigation|MovetoLocation (AI|GetAIController _self) _newlocation -1.0 true true false true 0)
        (Math|Integer|DecrementInt (Variables|Movement|GetmyRemainingMoveToActions)
          (:%20%20
            (Variables|State|SetmyIsWalking true)
            (Variables|Default|SetmyLastLocation (Transformation|GetWorldLocation (Variables|Collision|GetCapsuleComponent)))
            (Utilities|Time|SetTimerbyEvent (EventDispatchers|CreateEvent :!event Custom|CheckPosition) 1.0)
            (return)))
        (else
          (return))))
    (else
      (return))))

(fn OnReachedWalkPoint
  (Deciding|SetMovementWaitCooldown)
  (Variables|State|SetmyIsWalking false))

(fn SetMovementWaitCooldown
  (Variables|Movement|SetmyMovementWaitCooldown (Math|Random|RandomFloatinRange 4.0 6.5))
  (Variables|Movement|SetmyMovementWaitTimer 0.0))

(fn CancelMovetoPoint
  (Default|OnCatPickedUp (Variables|Default|GetmyCatManager) self)
  (Deciding|SetMovementWaitCooldown))

(fn PlayMeowSound
  (Audio|Components|Audio|SetSound (Variables|Default|GetAudio) (Utilities|Select :Index (Math|Random|RandomIntegerinRange 0 5) :Option%200 "/Game/Audio/SFX/SFX_Meow1.SFX_Meow1" :Option%201 "/Game/Audio/SFX/SFX_Meow2.SFX_Meow2" :Option%202 "/Game/Audio/SFX/SFX_Meow3.SFX_Meow3" :Option%203 "/Game/Audio/SFX/SFX_Meow4.SFX_Meow4" :Option%204 "/Game/Audio/SFX/SFX_Meow5.SFX_Meow5" :Option%205 "/Game/Audio/SFX/SFX_Meow6.SFX_Meow6"))
  (Audio|Components|Audio|Play (Variables|Default|GetAudio) 0.0)
  (Variables|Meow|SetmyMeowCooldown 2.0))

(fn SetMovementBlocked
  (params (newState :type Boolean))
  (Variables|State|SetmyMovementBlocked newState))