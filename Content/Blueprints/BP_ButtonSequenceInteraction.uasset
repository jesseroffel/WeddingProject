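; Interaction actor that has the player press a randomly generated sequence of gamepad face buttons to complete it.
; Construction builds the sequence, shifting any roll that repeats the previous button to the next one.
; A sphere overlap notifies player enter and exit and toggles tick, while TriggerInteract advances on correct presses and disables collision when finished.
; Getters expose the current key, up to three upcoming keys and completion progress.
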(event OnComponentBeginOverlap(SphereCollision)
  (params (OverlappedComponent :type Primitive%20Component%20Object%20Reference) (OtherActor :type Actor%20Object%20Reference) (OtherComp :type Primitive%20Component%20Object%20Reference) (OtherBodyIndex :type Integer) (bFromSweep :type Boolean) (SweepResult :type Hit%20Result%20Structure%20%28by%20ref%29))
  (bind _asbp_player_base (Utilities|Casting|CastToBP_PlayerBase OtherActor))
  (CallFunction|OnPlayerBeginOverlap _asbp_player_base)
  (Actor|Tick|SetActorTickEnabled true))

(event OnComponentEndOverlap(SphereCollision)
  (params (OverlappedComponent :type Primitive%20Component%20Object%20Reference) (OtherActor :type Actor%20Object%20Reference) (OtherComp :type Primitive%20Component%20Object%20Reference) (OtherBodyIndex :type Integer))
  (bind _asbp_player_base (Utilities|Casting|CastToBP_PlayerBase OtherActor))
  (CallFunction|OnPlayerEndOverlap _asbp_player_base)
  (if (CallFunction|IsFinished)
    (Collision|SetCollisionEnabled (Variables|Default|GetSphereCollision) "NoCollision")
    (else
      (Actor|Tick|SetActorTickEnabled false))))

(fn ConstructionScript
  (|CallParentFunction)
  (Variables|Default|SetmyInteractionType "NewEnumerator2")
  (CallFunction|SetupButtonSequence))

(fn GetButtonSequences
  (LocalVariables|SetsetCurrentKey (Utilities|Array|Get(acopy) (Variables|ButtonSequence|GetmyButtonSequence) (Variables|ButtonSequence|GetmyCurrentSequenceIndex)))
  (if (<= (+ (Variables|ButtonSequence|GetmyCurrentSequenceIndex) 1) (- (Utilities|Array|Length (Variables|ButtonSequence|GetmyButtonSequence)) 1))
    (LocalVariables|SetsetNextKey (Utilities|Array|Get(acopy) (Variables|ButtonSequence|GetmyButtonSequence) (+ (Variables|ButtonSequence|GetmyCurrentSequenceIndex) 1))))
  (if (<= (+ (Variables|ButtonSequence|GetmyCurrentSequenceIndex) 2) (- (Utilities|Array|Length (Variables|ButtonSequence|GetmyButtonSequence)) 1))
    (LocalVariables|SetsetSecondNextKey (Utilities|Array|Get(acopy) (Variables|ButtonSequence|GetmyButtonSequence) (+ (Variables|ButtonSequence|GetmyCurrentSequenceIndex) 2))))
  (if (<= (+ (Variables|ButtonSequence|GetmyCurrentSequenceIndex) 3) (- (Utilities|Array|Length (Variables|ButtonSequence|GetmyButtonSequence)) 1))
    (LocalVariables|SetsetThirdNextKey (Utilities|Array|Get(acopy) (Variables|ButtonSequence|GetmyButtonSequence) (+ (Variables|ButtonSequence|GetmyCurrentSequenceIndex) 3))))
  (return (LocalVariables|GetsetCurrentKey) (LocalVariables|GetsetNextKey) (LocalVariables|GetsetSecondNextKey) (LocalVariables|GetsetThirdNextKey)))

(fn TriggerInteract
  (params (PressedInput :type Key%20Structure))
  (if (== (Utilities|Array|Get(acopy) (Variables|ButtonSequence|GetmyButtonSequence) (Variables|ButtonSequence|GetmyCurrentSequenceIndex)) PressedInput)
    (Math|Integer|IncrementInt (Variables|ButtonSequence|GetmyCurrentSequenceIndex)
      (:%20%20
        (if (>= (Variables|ButtonSequence|GetmyCurrentSequenceIndex) (Utilities|Array|Length (Variables|ButtonSequence|GetmyButtonSequence)))
          (CallFunction|SetInteractionState "NewEnumerator5")
          (|CallParentFunction PressedInput)
          (Collision|SetCollisionEnabled (Variables|Default|GetSphereCollision) "NoCollision")
          (return true true)
          (else
            (|CallParentFunction PressedInput)
            (return true false)))))))

(fn GetButtonSequenceProcent
  (return (Math|Float|Clamp(Float) (/ (Math|Conversions|ToFloat(Integer) (Variables|ButtonSequence|GetmyCurrentSequenceIndex)) (Math|Conversions|ToFloat(Integer) (Utilities|Array|Length (Variables|ButtonSequence|GetmyButtonSequence)))))))

(fn SetupButtonSequence
  (while (< (Utilities|Array|Length (Variables|ButtonSequence|GetmyButtonSequence)) (Variables|ButtonSequence|GetmyButtonSequenceCount))
    (bind _output_get (LocalVariables|SetrolledButton (Math|Random|RandomIntegerinRange 0 3)))
    (LocalVariables|SetcurrentButtonRolled (Utilities|Select :Index _output_get :Option%200 "Gamepad_FaceButton_Bottom" :Option%201 "Gamepad_FaceButton_Right" :Option%202 "Gamepad_FaceButton_Top" :Option%203 "Gamepad_FaceButton_Left"))
    (if (> (LocalVariables|GetbuttonSequenceIndex) 0)
      (if (== (LocalVariables|GetcurrentButtonRolled) (Utilities|Array|Get(acopy) (Variables|ButtonSequence|GetmyButtonSequence) (- (LocalVariables|GetbuttonSequenceIndex) 1)))
        (if (> (+ (LocalVariables|GetrolledButton) 1) 3)
          (LocalVariables|SetrolledButton 0)
          (else
            (LocalVariables|SetrolledButton (+ (LocalVariables|GetrolledButton) 1))))
        (LocalVariables|SetcurrentButtonRolled (Utilities|Select :Index (LocalVariables|GetrolledButton) :Option%200 "Gamepad_FaceButton_Bottom" :Option%201 "Gamepad_FaceButton_Right" :Option%202 "Gamepad_FaceButton_Top" :Option%203 "Gamepad_FaceButton_Left"))))
    (Utilities|Array|Add (Variables|ButtonSequence|GetmyButtonSequence) (LocalVariables|GetcurrentButtonRolled))
    (Math|Integer|IncrementInt (LocalVariables|GetbuttonSequenceIndex))))