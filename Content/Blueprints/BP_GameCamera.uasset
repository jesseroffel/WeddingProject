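; BP_GameCamera is a shared camera that keeps two player characters in view.
; SetupCamera stores the player array and enables tracking.
; Each tick, the Sphere component lerps toward the players' average location, offset back and upward, by a fixed per-frame move-speed alpha.
; The spring arm length follows the distance between the first two players, clamped between minimum and maximum limits, so the camera zooms as they separate.
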(event EventTick
  (params (DeltaSeconds :type Float%20%28single-precision%29))
  (if (Variables|Default|GetmyGameStarted)
    (CallFunction|SetWorldLocation)
    (Variables|/Script/Engine.SpringArmComponent|SetTargetArmLength (Variables|Default|GetSpringArm) (Math|Float|Clamp(Float) (Transformation|GetDistanceTo (Utilities|Array|Get(acopy) (Variables|Default|GetmyPlayerCharacters)) (Utilities|Array|Get(acopy) (Variables|Default|GetmyPlayerCharacters) 1)) (Variables|Default|GetmyMinCamDistance) (Variables|Default|GetmyMaxCamDistance)))))

(fn ConstructionScript)

(fn SetupCamera
  (params (Players :type Array%20of%20BP%20Player%20Base%20Object%20References))
  (Variables|Default|SetmyPlayerCharacters Players)
  (Variables|Default|SetmyGameStarted true))

(fn SetWorldLocation
  (Variables|Default|SetmyPreviousLocation (Transformation|GetWorldLocation (Variables|Default|GetSphere)))
  (bind _returnvalue (Class|GameplayStatics|GetActorArrayAverageLocation (Variables|Default|GetmyPlayerCharacters)))
  (Transformation|SetWorldLocation (Variables|Default|GetSphere) (Math|Vector|Lerp(Vector) (Variables|Default|GetmyPreviousLocation) (Math|Vector|MakeVector (- (.X (Math|Vector|BreakVector _returnvalue)) 225.0) (.Y (Math|Vector|BreakVector _returnvalue)) (+ (.Z (Math|Vector|BreakVector _returnvalue)) 1.5e+02)) (Variables|Default|GetmyMoveSpeed)) false false))