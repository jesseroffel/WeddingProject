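; Progression manager that drives music and voicemails from the share of BP_InteractionBase actors the player has finished.
; Once started, Tick counts finished interactables, advances the music cue at fixed percentage steps and raises completion events.
; Timers switch loopable cues to their loop section through the LoopSelect sound parameter.
; Completion thresholds trigger up to three delayed voicemails, halving music volume until each ends.
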(event Custom|HandleInteractionProgression
  (CallFunction|CheckCompletedInteractables))

(event Custom|CheckVoicemail
  (params (deltaTime :type Float%20%28single-precision%29))
  (Voicemail|IncomingVoicemail deltaTime))

(event Custom|OnVoicemailFinished
  (Audio|Components|Audio|SetVolumeMultiplier (Variables|Default|GetMusic) 1.0 :!class /Script/Engine.AudioComponent))

(event Custom|HandleMusicLoop
  (params (DeltaTime :type Float%20%28single-precision%29))
  (if (< (Variables|Music|GetmyMusicCueStage) 6)
    (if (and (Utilities|Array|Get(acopy) (Variables|Music|GetmyAudioCanLoop) (Variables|Music|GetmyMusicCueStage)) (> (Variables|Music|GetmyRequiredAudioLoopTimer) 0.0))
      (bind _output_get (Variables|Music|SetmyAudioLoopTimer (+ (Variables|Music|GetmyAudioLoopTimer) DeltaTime)))
      (if (>= _output_get (Variables|Music|GetmyRequiredAudioLoopTimer))
        (Music|SwitchMusicLoop)))))

(event EventBeginPlay
  (bind _outactors (Actor|GetAllActorsOfClass "/Game/Blueprints/BP_InteractionBase.BP_InteractionBase_C"))
  (bind _output_get (Variables|Default|SetmyAllInteractables _outactors))
  (Variables|Default|SetmyTotalInterableCount (Utilities|Array|Length _output_get))
  (bind _output_get_2 (Variables|Music|SetmyMusicInteractStep 0.15))
  (Variables|Music|SetmyMusicCuePercentage _output_get_2)
  (EventDispatchers|BindEventtoOnAudioFinished (Variables|Default|GetVoicemail) (delegate Custom|OnVoicemailFinished)))

(event EventTick
  (params (DeltaSeconds :type Float%20%28single-precision%29))
  (if (Variables|Default|GetmyGameStarted)
    (CallFunction|HandleInteractionProgression)
    (CallFunction|HandleMusicLoop DeltaSeconds)
    (CallFunction|CheckVoicemail DeltaSeconds)))

(fn ConstructionScript)

(fn CheckCompletedInteractables
  (for _array_element (Variables|Default|GetmyAllInteractables)
    (if (Default|IsFinished _array_element)
      (Math|Integer|IncrementInt (LocalVariables|GetmyFinishedInteractables))))
  (if (> (LocalVariables|GetmyFinishedInteractables) (Variables|Default|GetmyCompletedInteractables))
    (bind _output_get (Variables|Default|SetmyCompletedInteractables (LocalVariables|GetmyFinishedInteractables)))
    (if (>= (/ (Math|Conversions|ToFloat(Integer) _output_get) (Math|Conversions|ToFloat(Integer) (Variables|Default|GetmyTotalInterableCount))) (Variables|Music|GetmyMusicCuePercentage))
      (Math|Integer|IncrementInt (Variables|Music|GetmyMusicCueStage)
        (:%20%20
          (Music|SwitchMusicCue)
          (Variables|Music|SetmyMusicCuePercentage (+ (Variables|Music|GetmyMusicInteractStep) (Variables|Music|GetmyMusicCuePercentage))))))
    (Default|CallOnInteractionCompleted _output_get)))

(fn HandleInteractableProgress
  (bind _mystageprogression (Variables|Default|GetmyStageProgression))
  (bind _output_get (LocalVariables|SetprogressPercentage (/ (Math|Conversions|ToFloat(Integer) (Variables|Default|GetmyCompletedInteractables)) (Math|Conversions|ToFloat(Integer) (Variables|Default|GetmyTotalInterableCount)))))
  (Development|PrintString (Utilities|String|ToString(Float) _output_get))
  (bind _result (Math|Integer|IncrementInt (Variables|Default|GetmyStageProgression))
    (:%20%20
      (Default|CallOnInteractionStageIncrease _result)
      (if (Math|Boolean|ORBoolean (== _mystageprogression 0) (== _mystageprogression 3) (== _mystageprogression 7))
        (Variables|Voicemail|SetmyVoicemailDelay 2.0)
        (Development|PrintString (Utilities|String|Append "Voicemail delay for stage progression: " (Utilities|String|ToString(Integer) _mystageprogression)))))))

(fn SwitchMusicCue
  (if (< (Variables|Music|GetmyMusicCueStage) (Variables|Music|GetmyMaxMusicCues))
    (Audio|Components|Audio|SetSound (Variables|Default|GetMusic) (Utilities|Array|Get(acopy) (Variables|Music|GetmySoundCues) (Variables|Music|GetmyMusicCueStage)))
    (if (Utilities|Array|Get(acopy) (Variables|Music|GetmyAudioCanLoop) (Variables|Music|GetmyMusicCueStage))
      (Effects|Components|ParticleSystem|SetIntParameter (Variables|Default|GetMusic) "LoopSelect" 0))
    (Audio|Components|Audio|Play (Variables|Default|GetMusic) 0.0)
    (bind _output_get (Variables|Music|SetmyRequiredAudioLoopTimer (Utilities|Array|Get(acopy) (Variables|Music|GetmyAudioLoopDelayDurations) (Variables|Music|GetmyMusicCueStage))))
    (Variables|Music|SetmyAudioLoopTimer 0.0)
    (Development|PrintString (Utilities|String|Append "Cue: " (Utilities|GetObjectName (Utilities|Array|Get(acopy) (Variables|Music|GetmySoundCues) (Variables|Music|GetmyMusicCueStage))) ", Delay: " (Utilities|String|ToString(Float) _output_get)))))

(fn IncomingVoicemail
  (params (DeltaTime :type Float%20%28single-precision%29))
  (bind _voicemail (Variables|Default|GetVoicemail))
  (bind _myvoicemailcounter (Variables|Voicemail|GetmyVoicemailCounter))
  (if (< (Variables|Voicemail|GetmyVoicemailCounter) 3)
    (if (>= (/ (Math|Conversions|ToFloat(Integer) (Variables|Default|GetmyCompletedInteractables)) (Math|Conversions|ToFloat(Integer) (Variables|Default|GetmyTotalInterableCount))) (Utilities|Array|Get(acopy) (Variables|Voicemail|GetmyVoicemailTriggerPercentages) (Variables|Voicemail|GetmyVoicemailCounter)))
      (bind _output_get (Variables|Voicemail|SetmyVoicemailDelayTimer (+ (Variables|Voicemail|GetmyVoicemailDelayTimer) DeltaTime)))
      (if (> _output_get (Variables|Voicemail|GetmyVoicemailDelay))
        (Development|PrintString (Utilities|String|Append "Play Voicemail: " (Utilities|String|ToString(Integer) _myvoicemailcounter)))
        (Effects|Components|ParticleSystem|SetIntParameter _voicemail "Voicemail" _myvoicemailcounter)
        (Audio|Components|Audio|SetVolumeMultiplier (Variables|Default|GetMusic) 0.5 :!class /Script/Engine.AudioComponent)
        (Audio|Components|Audio|Play _voicemail 0.0)
        (Default|CallOnVoicemailStart (Variables|Voicemail|GetmyVoicemailCounter))
        (Math|Integer|IncrementInt (Variables|Voicemail|GetmyVoicemailCounter)
          (:%20%20
            (Variables|Voicemail|SetmyVoicemailDelay 0.0)
            (Variables|Voicemail|SetmyVoicemailDelayTimer 0.0)))))))

(fn StartGame
  (Variables|Default|SetmyGameStarted true))

(fn StartPlayers
  (Music|SwitchMusicCue))

(fn SwitchMusicLoop
  (Effects|Components|ParticleSystem|SetIntParameter (Variables|Default|GetMusic) "LoopSelect" 1)
  (Development|PrintString "Switch to loop")
  (Variables|Music|SetmyRequiredAudioLoopTimer -1.0)
  (Variables|Music|SetmyAudioLoopTimer 0.0))