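; BP_PlateStorage is a storage station for clean dishes, derived from a parent that handles receiving pickup items.
; The construction script sets its required pickup type to BP_CleanDishes.
; When the total items are received, it runs the parent logic, plays a plate-moving sound and starts a one-shot timer matching the sound's duration.
; The OnPlatesMovingDone event swaps the shelf mesh to its completed version.
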(event Custom|OnPlatesMovingDone
  (Components|StaticMesh|SetStaticMesh (Variables|Default|GetShelf) "/Game/Props/Interactable/SM_Shelf_completed.SM_Shelf_completed"))

(fn ConstructionScript
  (|CallParentFunction)
  (Variables|Default|SetmyRequiredPickupType "/Game/Blueprints/BP_CleanDishes.BP_CleanDishes_C"))

(fn OnTotalItemsReceived
  (bind _audio (Variables|Default|GetAudio))
  (|CallParentFunction)
  (Audio|Components|Audio|SetSound _audio "/Game/Audio/SFX/SFX_PlatesMoving.SFX_PlatesMoving")
  (Audio|Components|Audio|Play _audio 0.0)
  (Utilities|Time|SetTimerbyEvent (EventDispatchers|CreateEvent :!event Custom|OnPlatesMovingDone) (Variables|/Script/Engine.SoundBase|GetDuration (Variables|/Script/Engine.AudioComponent|GetSound _audio))))