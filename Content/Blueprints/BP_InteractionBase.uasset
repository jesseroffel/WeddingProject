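; Base Blueprint for interactables tied to a required player type, with an interaction type, face-button sequence and joystick direction.
; Overlap events track one character at a time and show or hide a W_Interaction widget, set up on first use.
; TriggerInteract forwards button input to that widget and always returns false.
; An enum state drives interactable and finished checks; SetInteractionState calls the empty OnCompleted hook for finished states, never OnFinished.
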(event Custom|OnPlayerBeginOverlap
  (params (Player :type BP%20Player%20Base%20Object%20Reference))
  ;[1 1 1] Player Begin/End Overlap
  (if (not (Utilities|IsValid (Variables|Default|GetmyInteractingCharacter)))
    (Variables|Default|SetmyInteractingCharacter Player)
    (bind _isfinished (CallFunction|IsFinished))
    (if (not _isfinished)
      (if (Utilities|IsValid (Variables|Widget|GetmyWidgetInteractionRef))
        _
        (else
          (CallFunction|SetupWidgetInteraction)))
      (Default|OnPlayerBeginOverlap (Variables|Widget|GetmyWidgetInteractionRef) (Variables|/Game/Blueprints/BP_PlayerBase.BP_PlayerBase_C|GetmyPlayerType (Variables|Default|GetmyInteractingCharacter)))
      (Development|SetHiddeninGame (Variables|Default|GetWidget) false false))))

(event Custom|OnPlayerEndOverlap
  (params (Player :type BP%20Player%20Base%20Object%20Reference))
  ;[1 1 1] Player Begin/End Overlap
  (if (== Player (Variables|Default|GetmyInteractingCharacter))
    (bind _asw_interaction (Utilities|Casting|CastToW_Interaction (UserInterface|GetWidget (Variables|Default|GetWidget))))
    (Default|OnPlayerEndOverlap _asw_interaction)
    (Development|SetHiddeninGame (Variables|Default|GetWidget) true false)
    (Variables|Default|SetmyInteractingCharacter 0)))

(event Custom|OnInteractStart
  (Default|OnInteractionStart (Variables|Widget|GetmyWidgetInteractionRef))
  (Development|PrintString (Utilities|String|Append "Interaction: " (Utilities|String|Append (Utilities|GetDisplayName self) (Utilities|String|Append ",  Type: " (Utilities|String|EnumtoString (Variables|Default|GetmyInteractionType)))))))

(event Custom|SetupWidgetInteraction
  ;[1 1 1] Setup Widget
  (bind _asw_interaction (Utilities|Casting|CastToW_Interaction (UserInterface|GetWidget (Variables|Default|GetWidget))))
  (bind _output_get (Variables|Widget|SetmyWidgetInteractionRef _asw_interaction))
  (Default|OnSetup _output_get self (Variables|Default|GetmyRequiredPlayer)))

(fn ConstructionScript)

(fn TriggerInteract
  (params (PressedInput :type Key%20Structure :default "None"))
  (bind _mywidgetinteractionref (Variables|Widget|GetmyWidgetInteractionRef))
  (if (Utilities|IsValid _mywidgetinteractionref)
    (Default|OnInteractionButton _mywidgetinteractionref PressedInput))
  (return false false))

(fn IsInteractable
  (params (RequiredPlayer :type E_RequiredPlayer%20Enum :default "NewEnumerator0"))
  (bind _mycurrentinteractionstate (Variables|Default|GetmyCurrentInteractionState))
  (if (Utilities|Enum|Equal(Enum) RequiredPlayer (Variables|Default|GetmyRequiredPlayer))
    (return (and (and (Utilities|Enum|NotEqual(Enum) _mycurrentinteractionstate "NewEnumerator0") (Utilities|Enum|NotEqual(Enum) _mycurrentinteractionstate "NewEnumerator4")) (and (Utilities|Enum|NotEqual(Enum) _mycurrentinteractionstate "NewEnumerator3") (Utilities|Enum|NotEqual(Enum) _mycurrentinteractionstate "NewEnumerator5"))))
    (else
      (return false))))

(fn IsFinished
  (bind _mycurrentinteractionstate (Variables|Default|GetmyCurrentInteractionState))
  (return (or (Utilities|Enum|Equal(Enum) _mycurrentinteractionstate "NewEnumerator0") (Utilities|Enum|Equal(Enum) _mycurrentinteractionstate "NewEnumerator5"))))

(fn IsCompleted
  (return (Utilities|Enum|Equal(Enum) (Variables|Default|GetmyCurrentInteractionState) "NewEnumerator5")))

(fn SetInteractionState
  (params (NewInteractionState :type E_InteractionState%20Enum :default "NewEnumerator0"))
  (Variables|Default|SetmyCurrentInteractionState NewInteractionState)
  (bind _iscompleted (CallFunction|IsCompleted))
  (if _iscompleted
    (CallFunction|OnCompleted)
    (else
      (bind _isfinished (CallFunction|IsFinished))
      (if _isfinished
        (CallFunction|OnCompleted)))))

(fn OnFinished
  (return))

(fn OnCompleted
  (return))

(fn GetInteractionType
  (return (Variables|Default|GetmyInteractionType)))

(fn GetFaceButtonSequence
  (return (Variables|SequenceMinigame|GetmyFaceButtonSequence)))

(fn GetJoystickDirection
  (return (Variables|JoystickMinigame|GetmyJoystickDirection)))