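; BP_WaterPlant is an interactable plant-watering objective, built on parent interaction logic.
; It passes its sphere component to that logic as MySphereCollision and forwards overlap begin and end events.
; Starting the interaction plays watering audio.
; Completion stops the audio, disables the sphere's collision, swaps in the completed plant mesh and marks the objective complete on the HUD through GM_MainGameMode.
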(event OnComponentBeginOverlap(SphereCollision)
  (params (OverlappedComponent :type Primitive%20Component%20Object%20Reference) (OtherActor :type Actor%20Object%20Reference) (OtherComp :type Primitive%20Component%20Object%20Reference) (OtherBodyIndex :type Integer) (bFromSweep :type Boolean) (SweepResult :type Hit%20Result%20Structure%20%28by%20ref%29))
  (CallFunction|OnBeginOverlap OtherActor))

(event OnComponentEndOverlap(SphereCollision)
  (params (OverlappedComponent :type Primitive%20Component%20Object%20Reference) (OtherActor :type Actor%20Object%20Reference) (OtherComp :type Primitive%20Component%20Object%20Reference) (OtherBodyIndex :type Integer))
  (CallFunction|OnEndOverlap OtherActor))

(event EventBeginPlay
  (Variables|Default|SetmySphereCollision (Variables|Default|GetSphereCollision)))

(fn ConstructionScript
  (|CallParentFunction))

(fn OnInteractionStart
  (|CallParentFunction)
  (Audio|Components|Audio|SetSound (Variables|Default|GetAudio) "/Game/Audio/SFX/SQ_WateringPlants.SQ_WateringPlants")
  (Audio|Components|Audio|Play (Variables|Default|GetAudio) 0.0))

(fn OnInteractionCompleted
  (|CallParentFunction)
  (Audio|Components|Audio|Stop (Variables|Default|GetAudio))
  (Collision|SetCollisionEnabled (Variables|Default|GetSphereCollision) "NoCollision")
  (Components|StaticMesh|SetStaticMesh (Variables|Default|GetPlantsMesh) "/Game/Props/Interactable/SM_Plant_Completed.SM_Plant_Completed")
  (bind _asgm_main_game_mode (Utilities|Casting|CastToGM_MainGameMode (Game|GetGameMode)))
  (Default|ObjectiveUpdateHUD _asgm_main_game_mode "NewEnumerator8" true))