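; BP_ItemDestinationBase is a base drop-off point where players deliver a required pickup type to complete an objective.
; On collision overlap, a player holding a matching item, and not the cat, increments the provided count and has OnDeliveredItem called.
; Once the count reaches the required amount, it disables its collision and tells GM_MainGameMode to mark its objective type complete on the HUD.
; IsCompleted exposes whether the requirement is met.
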(event OnComponentBeginOverlap(Collision)
  (params (OverlappedComponent :type Primitive%20Component%20Object%20Reference) (OtherActor :type Actor%20Object%20Reference) (OtherComp :type Primitive%20Component%20Object%20Reference) (OtherBodyIndex :type Integer) (bFromSweep :type Boolean) (SweepResult :type Hit%20Result%20Structure%20%28by%20ref%29))
  (bind _asbp_player_base (Utilities|Casting|CastToBP_PlayerBase OtherActor))
  (if (and (Default|GetIsHoldingItem _asbp_player_base) (not (Default|GetIsHoldingCat _asbp_player_base)))
    (if (== (Utilities|GetClass (Default|GetHeldItem _asbp_player_base)) (Variables|Default|GetmyRequiredPickupType))
      (CallFunction|OnItemProvided)
      (Default|OnDeliveredItem _asbp_player_base))))

(fn ConstructionScript)

(fn OnItemProvided
  (Math|Integer|IncrementInt (Variables|Default|GetmyItemsProvided)
    (:%20%20
      (if (>= (Variables|Default|GetmyItemsProvided) (Variables|Default|GetmyItemsRequired))
        (CallFunction|OnTotalItemsReceived)))))

(fn OnTotalItemsReceived
  (Collision|SetCollisionEnabled (Variables|Default|GetCollision) "NoCollision")
  (bind _asgm_main_game_mode (Utilities|Casting|CastToGM_MainGameMode (Game|GetGameMode)))
  (Default|ObjectiveUpdateHUD _asgm_main_game_mode (Variables|Default|GetmyObjectiveType) true))

(fn IsCompleted
  (return (>= (Variables|Default|GetmyItemsProvided) (Variables|Default|GetmyItemsRequired))))