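; Flower pot interactable, derived from a parent interactable, that a cat can break and that can then be fixed.
; When targeted, it enables cat collision and notifies the cat on arrival.
; Parent hook overrides swap intact and broken meshes, toggle collisions and play matching sounds, with a timer following the break sound.
; Completing the fix notifies the stored cat and disables the interaction box.
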(event OnComponentBeginOverlap(BoxCollision)
  (params (OverlappedComponent :type Primitive%20Component%20Object%20Reference) (OtherActor :type Actor%20Object%20Reference) (OtherComp :type Primitive%20Component%20Object%20Reference) (OtherBodyIndex :type Integer) (bFromSweep :type Boolean) (SweepResult :type Hit%20Result%20Structure%20%28by%20ref%29))
  (CallFunction|OnBeginOverlap OtherActor))

(event OnComponentEndOverlap(BoxCollision)
  (params (OverlappedComponent :type Primitive%20Component%20Object%20Reference) (OtherActor :type Actor%20Object%20Reference) (OtherComp :type Primitive%20Component%20Object%20Reference) (OtherBodyIndex :type Integer))
  (CallFunction|OnEndOverlap OtherActor))

(event OnComponentBeginOverlap(CatCollision)
  (params (OverlappedComponent :type Primitive%20Component%20Object%20Reference) (OtherActor :type Actor%20Object%20Reference) (OtherComp :type Primitive%20Component%20Object%20Reference) (OtherBodyIndex :type Integer) (bFromSweep :type Boolean) (SweepResult :type Hit%20Result%20Structure%20%28by%20ref%29))
  (bind _asbp_cat_base (Utilities|Casting|CastToBP_CatBase OtherActor))
  (if (Variables|Default|GetmyIsTargetted)
    (Variables|Default|SetmyIsTargetted false)
    (Default|OnCatInteractableReached _asbp_cat_base)))

(event Custom|PlayDestroyNotificationSound
  (Audio|Components|Audio|SetSound (Variables|Default|GetAudio) "/Game/Audio/SFX/SFX_CatDestroyHappened.SFX_CatDestroyHappened")
  (Audio|Components|Audio|Play (Variables|Default|GetAudio) 0.0))

(event EventBeginPlay
  (|CallParentFunction)
  (Variables|Default|SetmyBoxCollision (Variables|Default|GetBoxCollision)))

(fn ConstructionScript
  (|CallParentFunction)
  (Variables|Default|SetmyCurrentInteractionState "NewEnumerator5"))

(fn OnCatDestroy
  (params (TargettingCat :type BP%20Cat%20Base%20Object%20Reference))
  (bind _plantpotbroken (Variables|Default|GetPlantPotBroken))
  (Variables|Default|SetmyTargettingCat TargettingCat)
  (Audio|Components|Audio|SetSound (Variables|Default|GetAudio) "/Game/Audio/SFX/SFX_FlowerPotBreak.SFX_FlowerPotBreak")
  (Audio|Components|Audio|Play (Variables|Default|GetAudio) 0.0)
  (Rendering|SetVisibility (Variables|Default|GetPlantPotComplete) false false)
  (Rendering|SetVisibility _plantpotbroken true false)
  (Collision|SetCollisionEnabled _plantpotbroken "QueryOnly")
  (CallFunction|SetInteractionState "NewEnumerator1")
  (CallFunction|OnResetInteraction)
  (Collision|SetCollisionEnabled (Variables|Default|GetBoxCollision) "QueryAndPhysics")
  (Collision|SetCollisionEnabled (Variables|Default|GetCatCollision) "NoCollision")
  (Utilities|Time|SetTimerbyEvent (EventDispatchers|CreateEvent :!event Custom|PlayDestroyNotificationSound) (Variables|/Script/Engine.SoundBase|GetDuration (Variables|/Script/Engine.AudioComponent|GetSound (Variables|Default|GetAudio))))
  (|CallParentFunction 0))

(fn OnInteractionStart
  (|CallParentFunction)
  (Audio|Components|Audio|SetSound (Variables|Default|GetAudio) "/Game/Audio/SFX/SQ_FlowerPotFixing.SQ_FlowerPotFixing")
  (Audio|Components|Audio|Play (Variables|Default|GetAudio) 0.0))

(fn OnInteractionCompleted
  (bind _plantpotbroken (Variables|Default|GetPlantPotBroken))
  (|CallParentFunction)
  (Audio|Components|Audio|SetSound (Variables|Default|GetAudio) "/Game/Audio/SFX/SFX_FlowerPotFixed.SFX_FlowerPotFixed")
  (Audio|Components|Audio|Play (Variables|Default|GetAudio) 0.0)
  (Rendering|SetVisibility (Variables|Default|GetPlantPotComplete) true false)
  (Rendering|SetVisibility _plantpotbroken false false)
  (Collision|SetCollisionEnabled _plantpotbroken "NoCollision")
  (if (Utilities|IsValid (Variables|Default|GetmyTargettingCat))
    (Default|OnTargettedInteractionCompleted (Variables|Default|GetmyTargettingCat))
    (Variables|Default|SetmyTargettingCat 0)
    (Collision|SetCollisionEnabled (Variables|Default|GetBoxCollision) "NoCollision")))

(fn OnCatTargetted
  (|CallParentFunction)
  (Collision|SetCollisionEnabled (Variables|Default|GetCatCollision) "QueryAndPhysics"))

(fn OnTimedReactivationStart
  (|CallParentFunction)
  (Audio|Components|Audio|SetSound (Variables|Default|GetAudio) "/Game/Audio/SFX/SQ_FlowerPotFixing.SQ_FlowerPotFixing")
  (Audio|Components|Audio|Play (Variables|Default|GetAudio) 0.0))