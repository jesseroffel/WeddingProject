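; Cake-baking oven interactable that uses its parent's timed reactivation to turn a placed Cake component into a BP_ItemCake.
; Box overlaps feed the parent's begin/end handlers, with end overlap ignored in one interaction state.
; Starting hides the cake, disables collision and plays the start sound, using its duration to time a follow-up event, apparently the oven loop.
; Finishing plays the end sound, spawns the item at the cake's transform and hides the widget.
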(event OnComponentBeginOverlap(BoxCollision)
  (params (OverlappedComponent :type Primitive%20Component%20Object%20Reference) (OtherActor :type Actor%20Object%20Reference) (OtherComp :type Primitive%20Component%20Object%20Reference) (OtherBodyIndex :type Integer) (bFromSweep :type Boolean) (SweepResult :type Hit%20Result%20Structure%20%28by%20ref%29))
  (CallFunction|OnBeginOverlap OtherActor))

(event OnComponentEndOverlap(BoxCollision)
  (params (OverlappedComponent :type Primitive%20Component%20Object%20Reference) (OtherActor :type Actor%20Object%20Reference) (OtherComp :type Primitive%20Component%20Object%20Reference) (OtherBodyIndex :type Integer))
  (if (not (Utilities|Enum|Equal(Enum) (Variables|Default|GetmyCurrentInteractionState) "NewEnumerator3"))
    (CallFunction|OnEndOverlap OtherActor)))

(event Custom|OnOvenLoop
  (Audio|Components|Audio|SetSound (Variables|Default|GetAudio) "/Game/Audio/SFX/SQ_OvenLoop.SQ_OvenLoop")
  (Audio|Components|Audio|Play (Variables|Default|GetAudio) 0.0))

(event EventBeginPlay
  (Variables|Default|SetmyBoxCollision (Variables|Default|GetBoxCollision)))

(fn ConstructionScript
  (|CallParentFunction)
  (Variables|Default|SetmyCompletionType "NewEnumerator1")
  (Variables|Default|SetmyCooldown (Variables|Default|GetmyReactivateCooldown)))

(fn OnTimedReactivationStart
  (|CallParentFunction)
  (Audio|Components|Audio|SetSound (Variables|Default|GetAudio) "/Game/Audio/SFX/SFX_OvenStart.SFX_OvenStart")
  (Audio|Components|Audio|Play (Variables|Default|GetAudio) 0.0)
  (Rendering|SetVisibility (Variables|Default|GetCake) false false)
  (Utilities|Time|SetTimerbyEvent (EventDispatchers|CreateEvent :!event Custom|OnOvenLoop) (Variables|/Script/Engine.SoundBase|GetDuration (Variables|/Script/Engine.AudioComponent|GetSound (Variables|Default|GetAudio))))
  (Collision|SetCollisionEnabled (Variables|Default|GetBoxCollision) "NoCollision"))

(fn OnTimedReactivationEnd
  (|CallParentFunction)
  (Audio|Components|Audio|SetSound (Variables|Default|GetAudio) "/Game/Audio/SFX/SFX_OvenEnd.SFX_OvenEnd")
  (Audio|Components|Audio|Play (Variables|Default|GetAudio) 0.0)
  (Game|SpawnActorfromClass "/Game/Blueprints/BP_ItemCake.BP_ItemCake_C" (Transformation|GetWorldTransform (Variables|Default|GetCake)) "AlwaysSpawn" 0 0)
  (Rendering|SetVisibility (Variables|Default|GetWidget) false false))