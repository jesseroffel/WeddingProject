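; BP_CatManager coordinates the level's cats, unblocking their movement at game start and handing out walk points and interaction objectives.
; Random walk points avoid the other cat's current one via an index array parallel to the cat list, effectively assuming two cats.
; Only one random interactable is targeted at a time, for one assigned cat.
; Picking up that cat clears the objective; any pickup resets the walk point at the cat's own index.
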(event Custom|OnStartGame
  ;[1 1 1] Start Game
  (for _array_element (Variables|Refs|GetmyCats)
    (Default|SetMovementBlocked _array_element false)))

(event Custom|OnResetObjective
  (Variables|Interactable|SetmyActiveInteraction 0)
  (Variables|Interactable|SetmyAssignedCat 0))

(event EventBeginPlay
  ;[1 1 1] Begin Play
  (bind _outactors (Actor|GetAllActorsOfClass "/Game/Blueprints/BP_CatBase.BP_CatBase_C"))
  (bind _output_get (Variables|Refs|SetmyCats _outactors))
  (for _array_element _output_get
    (Utilities|Array|Add (Variables|Walking|GetmyCatWalkActorLocationIndex) -1))
  (if (== (Utilities|Array|Length (Variables|Refs|GetmyCatWalkLocations)) 0)
    (Development|PrintString "ERROR: No cat walk points found!" true true "(R=1.000000,G=0.038396,B=0.000000,A=1.000000)" 5.0)))

(fn ConstructionScript)

(fn GetNewWalkLocation
  (params (RequestingCat :type BP%20Cat%20Base%20Object%20Reference))
  (if (> (Utilities|Array|Length (Variables|Refs|GetmyCatWalkLocations)) 0)
    (while (or (== (Utilities|Array|Get(acopy) (Variables|Walking|GetmyCatWalkActorLocationIndex) (.OtherCatIndex (CallFunction|GetOtherCatIndex RequestingCat))) (LocalVariables|GetlocationIndex)) (== (LocalVariables|GetlocationIndex) -1))
      (LocalVariables|SetlocationIndex (Math|Random|RandomIntegerinRange 0 (- (Utilities|Array|Length (Variables|Refs|GetmyCatWalkLocations)) 1))))
    (Utilities|Array|SetArrayElem (Variables|Walking|GetmyCatWalkActorLocationIndex) (CallFunction|GetCatIndex RequestingCat) (LocalVariables|GetlocationIndex))
    (Default|AssignCat (Utilities|Array|Get(acopy) (Variables|Refs|GetmyCatWalkLocations) (LocalVariables|GetlocationIndex)) RequestingCat)
    (return (Transformation|GetActorLocation (Utilities|Array|Get(acopy) (Variables|Refs|GetmyCatWalkLocations) (LocalVariables|GetlocationIndex))))
    (else
      (Development|PrintString "Invalid cat locations")
      (return (Transformation|GetWorldLocation (Variables|/Script/Engine.Character|GetCapsuleComponent RequestingCat))))))

(fn GetOtherCatIndex
  (params (RequestingCat :type BP%20Cat%20Base%20Object%20Reference))
  (for (_array_element _array_index) (Variables|Refs|GetmyCats)
    (if (!= _array_element RequestingCat)
      (return _array_element _array_index))))

(fn GetCatIndex
  (params (Requesting%20Cat :type BP%20Cat%20Base%20Object%20Reference))
  (for (_array_element _array_index) (Variables|Refs|GetmyCats)
    (if (== _array_element Requesting%20Cat)
      (return _array_index))))

(fn OnCatPickedUp
  (params (PickedCat :type BP%20Cat%20Base%20Object%20Reference))
  (if (== PickedCat (Variables|Interactable|GetmyAssignedCat))
    (if (Utilities|IsValid (Variables|Interactable|GetmyActiveInteraction))
      (Default|SetIsTargetted (Variables|Interactable|GetmyActiveInteraction) false))
    (CallFunction|OnResetObjective))
  (Default|Reset (Utilities|Array|Get(acopy) (Variables|Refs|GetmyCatWalkLocations) (CallFunction|GetCatIndex PickedCat))))

(fn GetInteractionObjective
  (params (RequestingCat :type BP%20Cat%20Base%20Object%20Reference))
  (if (and (not (Utilities|IsValid (Variables|Interactable|GetmyActiveInteraction))) (!= (Utilities|Array|Length (Variables|Interactable|GetMyCatInteractable)) 0))
    (bind _output_get (LocalVariables|SetselectedInteraction (Utilities|Array|Get(acopy) (Variables|Interactable|GetMyCatInteractable) (Math|Random|RandomIntegerinRange 0 (- (Utilities|Array|Length (Variables|Interactable|GetMyCatInteractable)) 1)))))
    (Variables|Interactable|SetmyAssignedCat RequestingCat)
    (Development|PrintString (Utilities|String|Append "Assigning Cat: " (Utilities|GetDisplayName RequestingCat) ", with Objective: " (Utilities|GetDisplayName (LocalVariables|GetselectedInteraction))) true true "(R=0.000000,G=0.660000,B=1.000000,A=1.000000)" 1e+01)
    (bind _output_get_2 (Variables|Interactable|SetmyActiveInteraction _output_get))
    (Default|SetIsTargetted _output_get_2 true)
    (return _output_get_2)
    (else
      (Development|PrintString "Interaction objective already active")
      (return 0))))