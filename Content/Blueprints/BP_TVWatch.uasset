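; BP_TVWatch is an interactable TV that the player can watch, built on a parent interaction class.
; Its box collision is handed to the parent on BeginPlay, and overlap events are forwarded to the parent's begin and end overlap handlers.
; Starting the interaction plays looping TV audio and switches the screen material to a show.
; Completing it stops the audio, restores the screen and disables the box collision, preventing further overlap triggers.
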(event OnComponentBeginOverlap(BoxCollision)
  (params (OverlappedComponent :type Primitive%20Component%20Object%20Reference) (OtherActor :type Actor%20Object%20Reference) (OtherComp :type Primitive%20Component%20Object%20Reference) (OtherBodyIndex :type Integer) (bFromSweep :type Boolean) (SweepResult :type Hit%20Result%20Structure%20%28by%20ref%29))
  (CallFunction|OnBeginOverlap OtherActor))

(event OnComponentEndOverlap(BoxCollision)
  (params (OverlappedComponent :type Primitive%20Component%20Object%20Reference) (OtherActor :type Actor%20Object%20Reference) (OtherComp :type Primitive%20Component%20Object%20Reference) (OtherBodyIndex :type Integer))
  (CallFunction|OnEndOverlap OtherActor))

(event EventBeginPlay
  (Variables|Default|SetmyBoxCollision (Variables|Default|GetBoxCollision)))

(fn ConstructionScript
  (|CallParentFunction))

(fn OnInteractionStart
  (|CallParentFunction)
  (Audio|Components|Audio|SetSound (Variables|Default|GetAudio) "/Game/Audio/SFX/SQ_TVLoop.SQ_TVLoop")
  (Audio|Components|Audio|Play (Variables|Default|GetAudio) 0.0)
  (Rendering|Material|SetMaterial (Variables|Default|GetTV) 1 "/Game/Props/Furnitures/Materials/MI_TVScreen_Show.MI_TVScreen_Show"))

(fn OnInteractionCompleted
  (|CallParentFunction)
  (Audio|Components|Audio|Stop (Variables|Default|GetAudio))
  (Rendering|Material|SetMaterial (Variables|Default|GetTV) 1 "/Game/Props/Furnitures/Materials/MI_TVScreen.MI_TVScreen")
  (Collision|SetCollisionEnabled (Variables|Default|GetBoxCollision) "NoCollision"))